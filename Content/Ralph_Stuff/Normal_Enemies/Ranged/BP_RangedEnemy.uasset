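; Ranged enemy that fires at the player on a RangedAttack event and destroys itself when damage drops Health to zero.
; LineTrace traces on the Camera channel toward the player character and spawns BP_Enemy_Shot at the enemy's location only if it hits BP_ThirdPersonCharacter.
; RangedAttack then waits briefly to destroy Projectile, but LineTrace sets that variable to None instead of the spawned shot.
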(event `Ranged Attack`
  (bind _projectile (`self.Projectile`))
  (`self.Line Trace`)
  (`KismetSystemLibrary.Delay` 1.0)
  (`/Engine/EditorBlueprintResources/StandardMacros.IsValid` _projectile
    (:`Is Valid`
      (`self.K2_DestroyActor` _projectile))))

(event `self.ReceiveAnyDamage`
  (params (Damage :type "Float (single-precision)") (DamageType :type "DamageType Object Reference") (InstigatedBy :type "Controller Object Reference") (DamageCauser :type "Actor Object Reference"))
  (bind _health (`self.Health`))
  (set `self.Health` (- _health Damage))
  (if (<= _health 0.0)
    (`self.K2_DestroyActor` self)))

(fn `Line Trace`
  (bind _outhit (`KismetSystemLibrary.LineTraceSingle` (`self.K2_GetActorLocation`) (`self.K2_GetActorLocation` (`GameplayStatics.GetPlayerCharacter` 0)) "TraceTypeQuery2" false (`|MakeArray` (`self.BP_RangedEnemy`) :!type "Actor Object Reference") "ForOneFrame" true (struct :`R` 1.0 :`A` 1.0) (struct :`G` 1.0 :`A` 1.0) 2.0))
  (cast `/Game/ThirdPerson/Blueprints/BP_ThirdPersonCharacter` (`.HitActor` (`GameplayStatics.BreakHitResult` _outhit)))
  (`|SpawnActorFromClass` "/Game/Ralph_Stuff/Normal_Enemies/Ranged/BP_Enemy_Shot.BP_Enemy_Shot_C" (`KismetMathLibrary.MakeTransform` (`self.K2_GetActorLocation`)) "Undefined" "MultiplyWithRoot" null null)
  (set `self.Projectile` null))

(fn `UserConstructionScript`)