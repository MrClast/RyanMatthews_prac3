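; BP_Enemy is a melee enemy, apparently a boss minion, that loses health from damage and is destroyed at zero.
; MinionAttack starts a punch montage and immediately sphere-traces between two socket components on the Camera channel, damaging the hit actor.
; It fires OnAttackEnd on a miss or player-character hit, but not for other actors.
; Sprint functions toggle walk speed; roll and stamina logic are empty or disconnected.
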(event `Minion Attack`
  (`|PlayMontage` (`self.Mesh`) "/Game/ryan_stuff/animations_testing/Paired_CounterPunch_PalmStrike_Att1_Montage.Paired_CounterPunch_PalmStrike_Att1_Montage"
    (:`then`
      (bind (_outhit _returnvalue) (`KismetSystemLibrary.SphereTraceSingle` :`Start` (`SceneComponent.GetSocketLocation` (`self.startmelee`) "None") :`End` (`SceneComponent.GetSocketLocation` (`self.endmelee`) "None") :`Radius` 30.0 :`TraceChannel` "TraceTypeQuery2" :`TraceColor` (struct :`G` 0.149324 :`B` 1.0 :`A` 1.0)))
      (if _returnvalue
        (bind (_bblockinghit _binitialoverlap _time _distance _location _impactpoint _normal _impactnormal _physmat _hitactor) (`GameplayStatics.BreakHitResult` _outhit))
        (`GameplayStatics.ApplyDamage` _hitactor 25.0)
        (cast `/Game/ThirdPerson/Blueprints/BP_ThirdPersonCharacter` _hitactor)
        (`self.OnAttackEnd`)
        (else
          (`self.OnAttackEnd`))))))

(event `self.ReceiveAnyDamage`
  (params (Damage :type "Float (single-precision)") (DamageType :type "DamageType Object Reference") (InstigatedBy :type "Controller Object Reference") (DamageCauser :type "Actor Object Reference"))
  ;[1 1 1] it dies
  (set `self.health` (- (`self.health`) Damage))
  (if (<= (`self.health`) 0.0)
    (`self.K2_DestroyActor` self)))

(fn `start roll`)

(fn `start sprinting`
  (set `CharacterMovementComponent.MaxWalkSpeed` 1000.0 (`self.CharacterMovement`)))

(fn `stop sprinting`
  (set `CharacterMovementComponent.MaxWalkSpeed` 400.0 (`self.CharacterMovement`)))

(fn `UserConstructionScript`)