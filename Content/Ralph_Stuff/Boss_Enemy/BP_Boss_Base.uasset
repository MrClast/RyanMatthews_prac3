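; Base boss enemy with a full-screen or HUD widget, sprint speed toggles, a melee attack and a homing missile swarm.
; Attack plays a punch montage and sphere-traces between melee points at start and completion to damage the player.
; LineTargeting traces to the player and spawns missiles in a random upward cone that home on them.
; At zero health it spawns BP_loadhub at its start point, removes the widget and destroys itself.
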(event `self.ReceiveBeginPlay`
  (set `self.startpoint` (`SceneComponent.K2_GetComponentLocation` (`self.Mesh`)))
  (bind _returnvalue (`|CreateWidget` "/Game/ryan_stuff/widgets/W_bossfull.W_bossfull_C"))
  (set `self.bossfull` _returnvalue)
  (`UserWidget.AddToViewport` _returnvalue 0))

(event `Attack`
  ;[1 0.4744 0.3259] The Attack Event for when the boss gets to the player it uses a montage to attack and shoot out a sphere trace to damage the player.
  (`|PlayMontage` (`self.Mesh`) "/Game/ryan_stuff/animations_testing/Paired_CounterPunch_PalmStrike_Att1_Montage.Paired_CounterPunch_PalmStrike_Att1_Montage" 1.0 0.0 "UpperBody"
    (:`then`
      _)
    (:`OnCompleted`
      _))
  (bind (_outhit _returnvalue) (`KismetSystemLibrary.SphereTraceSingle` :`Start` (`SceneComponent.GetSocketLocation` (`self.startmelee`) "None") :`End` (`SceneComponent.GetSocketLocation` (`self.endmelee`) "None") :`Radius` 30.0 :`TraceChannel` "TraceTypeQuery2" :`TraceColor` (struct :`G` 0.149324 :`B` 1.0 :`A` 1.0)))
  (if _returnvalue
    (bind (_bblockinghit _binitialoverlap _time _distance _location _impactpoint _normal _impactnormal _physmat _hitactor) (`GameplayStatics.BreakHitResult` _outhit))
    (bind _asbp_third_person_character (cast `/Game/ThirdPerson/Blueprints/BP_ThirdPersonCharacter` _hitactor))
    (`GameplayStatics.ApplyDamage` _asbp_third_person_character 25.0 null _hitactor)))

(event `self.ReceiveAnyDamage`
  (params (Damage :type "Float (single-precision)") (DamageType :type "DamageType Object Reference") (InstigatedBy :type "Controller Object Reference") (DamageCauser :type "Actor Object Reference"))
  ;[0.5878 0.2752 1] When damaged lose health.
  (set `self.health` (- (`self.health`) Damage))
  (if (<= (`self.health`) 0.0)
    (`|SpawnActorFromClass` "/Game/ryan_stuff/Ryan_DialogueStuff/BP_loadhub.BP_loadhub_C" (`KismetMathLibrary.Conv_VectorToTransform` (`self.startpoint`)) "Undefined" "MultiplyWithRoot" null null)
    (`Widget.RemoveFromParent` (`self.bossfull`))
    (`KismetSystemLibrary.CollectGarbage`)
    (`KismetSystemLibrary.Delay` 0.2)
    (`self.K2_DestroyActor` self)))

(fn `Calc Fire Point`
  (returns (ReturnValue :type "Vector Structure") (ReturnValue1 :type "Rotator Structure"))
  (bind _followcamera (`self.FollowCamera`))
  (bind _returnvalue (`SceneComponent.K2_GetComponentRotation` _followcamera))
  (return (+ (`SceneComponent.K2_GetComponentLocation` _followcamera) (* (`KismetMathLibrary.GetForwardVector` _returnvalue) (`SpringArmComponent.TargetArmLength` (`self.CameraBoom`)))) _returnvalue))

(fn `Find Player`
  ;[0.5583 0.3284 1] At the moment this is up in the air because all this does is add an arrow to the player. I would need an arrow and my targeting here so I could spawn an arrow on the player.
)

(fn `Fire Missile`
  (bind _returnvalue (`|SpawnActorFromClass` "/Game/Ralph_Stuff/Missile_Swarm/BP_SwarmMissile.BP_SwarmMissile_C" (`KismetMathLibrary.MakeTransform` (+ (`self.K2_GetActorLocation`) (0.0 0.0 150.0)) (`KismetMathLibrary.Conv_VectorToRotator` (`KismetMathLibrary.RandomUnitVectorInConeInDegrees` (0.0 0.0 1.0) 75.0))) "Undefined" "MultiplyWithRoot" null null))
  (set `ProjectileMovementComponent.HomingTargetComponent` (`Actor.RootComponent` (`self.Target`)) (`/Game/Ralph_Stuff/Missile_Swarm/BP_SwarmMissile.ProjectileMovement` _returnvalue)))

(fn `LineTargeting`
  (bind _returnvalue (+ (`self.K2_GetActorLocation`) (0.0 0.0 200.0)))
  (bind _outhit (`KismetSystemLibrary.LineTraceSingle` (`self.K2_GetActorLocation`) (`self.K2_GetActorLocation` (`GameplayStatics.GetPlayerCharacter` 0)) "TraceTypeQuery2" false (`|MakeArray` (`self.Boss`) :!type "Actor Object Reference") "ForOneFrame" true (struct :`G` 1.0 :`B` 0.04086 :`A` 1.0) (struct :`R` 1.0 :`G` 0.041839 :`A` 1.0)))
  (bind _asbp_third_person_character (cast `/Game/ThirdPerson/Blueprints/BP_ThirdPersonCharacter` (`.HitActor` (`GameplayStatics.BreakHitResult` _outhit))))
  (`GameplayStatics.PlaySoundAtLocation` "/Game/Ralph_Stuff/Missile_Swarm/spaceEngine_000.spaceEngine_000" _returnvalue (struct) 1.0 1.0 0.0 null null null null)
  (for _ (range (+ (`self.MissileCount`) 1))
    (bind _returnvalue_2 (`|SpawnActorFromClass` "/Game/Ralph_Stuff/Missile_Swarm/BP_SwarmMissile.BP_SwarmMissile_C" (`KismetMathLibrary.MakeTransform` _returnvalue (`KismetMathLibrary.Conv_VectorToRotator` (`KismetMathLibrary.RandomUnitVectorInConeInDegrees` (0.0 0.0 1.0) 75.0))) "Undefined" "MultiplyWithRoot" null null))
    (set `ProjectileMovementComponent.HomingTargetComponent` (`Actor.RootComponent` _asbp_third_person_character) (`/Game/Ralph_Stuff/Missile_Swarm/BP_SwarmMissile.ProjectileMovement` _returnvalue_2))))

(fn `start roll`)

(fn `start sprinting`
  (set `CharacterMovementComponent.MaxWalkSpeed` 1000.0 (`self.CharacterMovement`)))

(fn `stop sprinting`
  (set `CharacterMovementComponent.MaxWalkSpeed` 400.0 (`self.CharacterMovement`)))

(fn `UserConstructionScript`)