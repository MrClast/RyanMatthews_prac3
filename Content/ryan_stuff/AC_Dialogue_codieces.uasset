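; Dialogue component for Codieces, a talking book that converses with Laz, overriding Dialogue and branching on the tree index.
; Tree 0 plays the intro from DT_BookIntro, advancing one row per call.
; Tree 1 is a hardcoded return-visit menu of nested Adddialogue choices, with only the chat option branching further.
; Disconnected leftovers hold an older hardcoded intro, rat lines and the only calls that switch to tree 1.
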(fn `dialogue`
  (bind _array (`|MakeArray` "continue" :!type "Text"))
  (bind _array_2 (`|MakeArray` "continue" :!type "Text"))
  (`parent.dialogue`)
  (switch `int` (`self.dialoguetreeindex`)
    (:`0`
      ;[1 1 1] Comment
      (bind _outrownames (`DataTableFunctionLibrary.GetDataTableRowNames` "/Game/ryan_stuff/DT_BookIntro.DT_BookIntro"))
      (bind _returnvalue (`|GetDataTableRow` "/Game/ryan_stuff/DT_BookIntro.DT_BookIntro" (`|GetArrayItem` _outrownames (`self.currentDialogueLine`)))
        (:`then`
          (`self.adddialogue` (break `/Game/ryan_stuff/S_Dialogue` _returnvalue) (`.Dialogue_4_AD704CA54F6F1F72C9D01385E0AE3D27` (break `/Game/ryan_stuff/S_Dialogue` _returnvalue)) (`.SelectableOptions_8_06422B1545466DDC0A78A4832BCA00F4` (break `/Game/ryan_stuff/S_Dialogue` _returnvalue)))
          (`/Engine/EditorBlueprintResources/StandardMacros.IncrementInt` (`self.currentDialogueLine`) ; go to next row in data table
            (:`  `
              (`KismetSystemLibrary.PrintString` "updated row index"))))
        (:`RowNotFound`
          (`KismetSystemLibrary.PrintString` "end of dialogue"))))
    (:`1`
      (bind (_state _options_index) (`self.adddialogue` "Codieces" "Welcome back! What can I do for you today my friend? Perhaps a chat? Telling of old stories? Or better yet do you have any pages on you? " (`|MakeArray` "Chat" "pages" "ancient tales" :!type "Text")))
      (switch `/Game/ryan_stuff/Enum_Dialoguestate` _state
        (:`NewEnumerator0`
          (switch `int` _options_index
            (:`0`
              (bind (_state_2 _options_index_2) (`self.adddialogue` "Laz" "Just coming along for a chat, How are you holding up in the new home? " _array))
              (switch `/Game/ryan_stuff/Enum_Dialoguestate` _state_2
                (:`NewEnumerator0`
                  (switch `int` _options_index_2
                    (:`0`
                      (bind (_state_3 _options_index_3) (`self.adddialogue` "Codieces" "A chat is something I can handle. I'm holding up fine. Are you feeling okay lad? " (`|MakeArray` "just fine" "could be better" :!type "Text")))
                      (switch `/Game/ryan_stuff/Enum_Dialoguestate` _state_3
                        (:`NewEnumerator0`
                          (switch `int` _options_index_3
                            (:`0`
                              (bind (_state_4 _options_index_4) (`self.adddialogue` "Laz" "Holding up decently well. The arm is still something I will never be used to honestly." _array_2))
                              (switch `/Game/ryan_stuff/Enum_Dialoguestate` _state_4
                                (:`NewEnumerator0`
                                  (switch `int` _options_index_4
                                    (:`0`
                                      _)))))
                            (:`1`
                              (bind (_state_5 _options_index_5) (`self.adddialogue` "Laz" "Could be better, I think the arm is still giving me more trouble than necesssary though. " _array_2))
                              (switch `/Game/ryan_stuff/Enum_Dialoguestate` _state_5
                                (:`NewEnumerator0`
                                  (switch `int` _options_index_5
                                    (:`0`
                                      _))))))
                          (bind (_state_6 _options_index_6) (`self.adddialogue` "Codieces" "The arm huh? It's not very fleshy. I guess some injuries never heal properly huh? Nostradamus is quite the heavy hitter in a fight. " (`|MakeArray` "sure" "not for long" :!type "Text")))
                          (switch `/Game/ryan_stuff/Enum_Dialoguestate` _state_6
                            (:`NewEnumerator0`
                              (switch `int` _options_index_6
                                (:`0`
                                  (`self.adddialogue` "Laz" "Sure is. Always has been. But I wouldn't say hes stronger than me. "))
                                (:`1`
                                  (`self.adddialogue` "Laz" "Not for much longer, "))))))))))))
            (:`1`
              (`self.adddialogue` "Laz" "I think I have some pages here. I'll let you look at them. " _array))
            (:`2`
              (`self.adddialogue` "Laz" "I'd like to see some of the ancient tales you got in there. " _array))))))))