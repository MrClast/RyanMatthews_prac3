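; Boss base Blueprint, apparently a test variant, with a melee attack, health, taunts and sprint speed toggles.
; Attack plays a palm-strike montage and sphere-traces between melee points at start and completion, damaging the player character on hit.
; Damage reduces health, triggers quips only at exact thresholds and destroys the boss at zero.
; Quips briefly show random text on the player's widget; audio is disconnected and roll is empty.
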(event `Attack`
  (`|PlayMontage` (`self.Mesh`) "/Game/ryan_stuff/animations_testing/Paired_CounterPunch_PalmStrike_Att1_Montage.Paired_CounterPunch_PalmStrike_Att1_Montage"
    (:`then`
      _)
    (:`OnCompleted`
      _))
  (bind (_outhit _returnvalue) (`KismetSystemLibrary.SphereTraceSingle` :`Start` (`SceneComponent.GetSocketLocation` (`self.startmelee`) "None") :`End` (`SceneComponent.GetSocketLocation` (`self.endmelee`) "None") :`Radius` 30.0 :`TraceChannel` "TraceTypeQuery2" :`DrawDebugType` "ForDuration" :`TraceColor` (struct :`G` 0.149324 :`B` 1.0 :`A` 1.0)))
  (if _returnvalue
    (bind (_bblockinghit _binitialoverlap _time _distance _location _impactpoint _normal _impactnormal _physmat _hitactor) (`GameplayStatics.BreakHitResult` _outhit))
    (bind _asbp_third_person_character (cast `/Game/ThirdPerson/Blueprints/BP_ThirdPersonCharacter` _hitactor))
    (`GameplayStatics.ApplyDamage` _asbp_third_person_character 25.0 null _hitactor)
    (`KismetSystemLibrary.PrintString` "Damage")
    (`self.OnAttackEnd`)
    (else
      (`self.OnAttackEnd`))))

(event `self.ReceiveAnyDamage`
  (params (Damage :type "Float (single-precision)") (DamageType :type "DamageType Object Reference") (InstigatedBy :type "Controller Object Reference") (DamageCauser :type "Actor Object Reference"))
  (set `self.health` (- (`self.health`) Damage))
  (if (== (`self.health`) 400.0)
    (`self.quip`))
  (if (== (`self.health`) 300.0)
    (`self.quip`))
  (if (== (`self.health`) 200.0)
    (`self.quip`))
  (if (== (`self.health`) 100.0)
    (`self.quip`))
  (if (<= (`self.health`) 0.0)
    (`self.K2_DestroyActor` self)))

(event `quip`
  (bind _quiptext (`self.quiptext`))
  ;[1 1 1] not adding to viewport properly
  (bind _asbp_third_person_character (cast `/Game/ThirdPerson/Blueprints/BP_ThirdPersonCharacter` (`GameplayStatics.GetPlayerCharacter` 0)))
  (bind _bossquipwidget (`/Game/ThirdPerson/Blueprints/BP_ThirdPersonCharacter.bossquipwidget` _asbp_third_person_character))
  (`UserWidget.AddToViewport` _bossquipwidget 0)
  (`/Game/ryan_stuff/widgets/W_bossquip.updatebosstext` _bossquipwidget (`|GetArrayItem` _quiptext (`KismetMathLibrary.RandomIntegerInRange` 0 (- (`KismetArrayLibrary.Array_Length` _quiptext) 1))) (`self.bossname`))
  (`KismetSystemLibrary.Delay` 5.0)
  (`Widget.RemoveFromParent` _bossquipwidget))

(fn `start roll`)

(fn `start sprinting`
  (set `CharacterMovementComponent.MaxWalkSpeed` 1000.0 (`self.CharacterMovement`)))

(fn `stop sprinting`
  (set `CharacterMovementComponent.MaxWalkSpeed` 400.0 (`self.CharacterMovement`)))

(fn `UserConstructionScript`)