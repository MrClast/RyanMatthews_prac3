(fn `dialogue`
  (`parent.dialogue`)
  (switch `int` (`self.dialoguetreeindex`)
    (:`0`
      (bind (_state _options_index) (`self.adddialogue` "mouse" "Hello you got any cheese" (`|MakeArray` "Yes" "No" :!type "Text")))
      (switch `/Game/ryan_stuff/Enum_Dialoguestate` _state
        (:`NewEnumerator0`
          (switch `int` _options_index
            (:`0`
              (bind (_state_2 _options_index_2) (`self.adddialogue` "mouse" "Thats great news! can I have some?" (`|MakeArray` "give cheese" "keep cheese" :!type "Text")))
              (switch `/Game/ryan_stuff/Enum_Dialoguestate` _state_2
                (:`NewEnumerator0`
                  (switch `int` _options_index_2
                    (:`0`
                      (bind _state_3 (`self.adddialogue` "mouse" "Thank you You are so kind! " (`|MakeArray` "continue" :!type "Text")))
                      (switch `/Game/ryan_stuff/Enum_Dialoguestate` _state_3
                        (:`NewEnumerator0`
                          (`self.setdialoguetreeindex` 1)
                          (`self.closeconversation`))))
                    (:`1`
                      (bind _state_4 (`self.adddialogue` "mouse" "You kinda suck!" (`|MakeArray` "continue" :!type "Text")))
                      (switch `/Game/ryan_stuff/Enum_Dialoguestate` _state_4
                        (:`NewEnumerator0`
                          (`self.removedialogueprogress` 2)
                          (`self.closeconversation`))))))))
            (:`1`
              (bind _state_5 (`self.adddialogue` "mouse" "Thats a shame, i really wanted cheese" (`|MakeArray` "continue" :!type "Text")))
              (switch `/Game/ryan_stuff/Enum_Dialoguestate` _state_5
                (:`NewEnumerator0`
                  (`self.cleardialogueprogress`)
                  (`self.closeconversation`))))))))
    (:`1`
      (bind _state_6 (`self.adddialogue` "mouse" "Thanks for the cheese pal! " (`|MakeArray` "continue" :!type "Text")))
      (switch `/Game/ryan_stuff/Enum_Dialoguestate` _state_6
        (:`NewEnumerator0`
          (`self.cleardialogueprogress`)
          (`self.closeconversation`))))))