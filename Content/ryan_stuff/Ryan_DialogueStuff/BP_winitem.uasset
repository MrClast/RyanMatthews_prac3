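; BP_winitem is a win-condition trigger actor that shows the end-game screen when the player reaches it.
; On BeginPlay it creates the W_endgame widget and destroys the first NPC_Edward and NPC_codiieces actors it finds.
; Its Box overlap adds that widget to the viewport for actors tagged "player".
; An unconnected chain for a health-restoring pickup with a quip and sound never runs.
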(event `self.ReceiveBeginPlay`
  (bind _returnvalue (`|CreateWidget` "/Game/ryan_stuff/widgets/W_endgame.W_endgame_C"))
  (set `self.winscreen` _returnvalue)
  (bind _returnvalue_2 (`GameplayStatics.GetActorOfClass` "/Game/ryan_stuff/Ryan_DialogueStuff/NPC_Edward.NPC_Edward_C"))
  (`self.K2_DestroyActor` _returnvalue_2)
  (bind _returnvalue_3 (`GameplayStatics.GetActorOfClass` "/Game/ryan_stuff/Ryan_DialogueStuff/NPC_codiieces.NPC_codiieces_C"))
  (`self.K2_DestroyActor` _returnvalue_3))

(event `self.Box.OnComponentBeginOverlap`
  (params (OverlappedComponent :type "PrimitiveComponent Object Reference") (OtherActor :type "Actor Object Reference") (OtherComp :type "PrimitiveComponent Object Reference") (OtherBodyIndex :type Integer) (bFromSweep :type Boolean) (SweepResult :type "HitResult Structure (by ref)"))
  (if (`self.ActorHasTag` OtherActor "player")
    (`UserWidget.AddToViewport` (`self.winscreen`) 0)))

(fn `UserConstructionScript`)