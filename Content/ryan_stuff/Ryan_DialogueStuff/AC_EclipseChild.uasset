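; Dialogue component for the Eclipse Kid conversation, where Laz talks a child waiting in the mist for an eclipse into heading inside.
; Overrides the parent Dialogue function and, at tree index 0, runs a linear chain of Adddialogue calls, each with speaker, line, voice clip and a single response option.
; The final line resets the tree index to 0 and closes the conversation.
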(fn `dialogue`
  (`parent.dialogue`)
  (switch `int` (`self.dialoguetreeindex`)
    (:`0`
      (bind (_state _options_index) (`self.adddialogue` "Laz" "What are you doing out here kid?" (`|MakeArray` "Continue" :!type "Text") "/Game/ryan_stuff/Ryan_DialogueStuff/Audio/Eclipse_1.Eclipse_1"))
      (switch `/Game/ryan_stuff/Ryan_DialogueStuff/Enum_Dialoguestate` _state
        (:`NewEnumerator0`
          (switch `int` _options_index
            (:`0`
              (bind (_state_2 _options_index_2) (`self.adddialogue` "Eclipse Kid" "Waiting on the eclipse. " (`|MakeArray` "Uhhh" :!type "Text") "/Game/ryan_stuff/Ryan_DialogueStuff/Audio/Eclipse_2.Eclipse_2"))
              (switch `/Game/ryan_stuff/Ryan_DialogueStuff/Enum_Dialoguestate` _state_2
                (:`NewEnumerator0`
                  (switch `int` _options_index_2
                    (:`0`
                      (bind (_state_3 _options_index_3) (`self.adddialogue` "Laz" "Uhhh...with how misty it is out here, you're not going to see it. " (`|MakeArray` "Besides" :!type "Text") "/Game/ryan_stuff/Ryan_DialogueStuff/Audio/Eclipse_3.Eclipse_3"))
                      (switch `/Game/ryan_stuff/Ryan_DialogueStuff/Enum_Dialoguestate` _state_3
                        (:`NewEnumerator0`
                          (switch `int` _options_index_3
                            (:`0`
                              (bind (_state_4 _options_index_4) (`self.adddialogue` "Laz" "Besides, an eclipse hasn't been seen in any of the years I've been alive. It sure wont show up today. " (`|MakeArray` "continue" :!type "Text") "/Game/ryan_stuff/Ryan_DialogueStuff/Audio/Eclipse_4.Eclipse_4"))
                              (switch `/Game/ryan_stuff/Ryan_DialogueStuff/Enum_Dialoguestate` _state_4
                                (:`NewEnumerator0`
                                  (switch `int` _options_index_4
                                    (:`0`
                                      (bind (_state_5 _options_index_5) (`self.adddialogue` "Eclipse Kid" "Oh. That sucks. Well why are you out here mister Laz? " (`|MakeArray` "To drink" :!type "Text") "/Game/ryan_stuff/Ryan_DialogueStuff/Audio/Eclipse_5.Eclipse_5"))
                                      (switch `/Game/ryan_stuff/Ryan_DialogueStuff/Enum_Dialoguestate` _state_5
                                        (:`NewEnumerator0`
                                          (switch `int` _options_index_5
                                            (:`0`
                                              (bind (_state_6 _options_index_6) (`self.adddialogue` "Laz" "I like to drink where I can't be seen. " (`|MakeArray` "Continue" :!type "Text") "/Game/ryan_stuff/Ryan_DialogueStuff/Audio/Eclipse_6.Eclipse_6"))
                                              (switch `/Game/ryan_stuff/Ryan_DialogueStuff/Enum_Dialoguestate` _state_6
                                                (:`NewEnumerator0`
                                                  (switch `int` _options_index_6
                                                    (:`0`
                                                      (bind (_state_7 _options_index_7) (`self.adddialogue` "Eclipse Kid" "Well drinking isnt good for you. " (`|MakeArray` "Didn't know" :!type "Text") "/Game/ryan_stuff/Ryan_DialogueStuff/Audio/Eclipse_7.Eclipse_7"))
                                                      (switch `/Game/ryan_stuff/Ryan_DialogueStuff/Enum_Dialoguestate` _state_7
                                                        (:`NewEnumerator0`
                                                          (switch `int` _options_index_7
                                                            (:`0`
                                                              (bind (_state_8 _options_index_8) (`self.adddialogue` "Laz" "Gee. I didn't know. " (`|MakeArray` "Head inside" :!type "Text") "/Game/ryan_stuff/Ryan_DialogueStuff/Audio/Eclipse_8.Eclipse_8"))
                                                              (switch `/Game/ryan_stuff/Ryan_DialogueStuff/Enum_Dialoguestate` _state_8
                                                                (:`NewEnumerator0`
                                                                  (switch `int` _options_index_8
                                                                    (:`0`
                                                                      (bind (_state_9 _options_index_9) (`self.adddialogue` "Laz" "Why don't you head inside. The mist is turning more into a rain now." (`|MakeArray` "Continue" :!type "Text") "/Game/ryan_stuff/Ryan_DialogueStuff/Audio/Eclipse_9.Eclipse_9"))
                                                                      (switch `/Game/ryan_stuff/Ryan_DialogueStuff/Enum_Dialoguestate` _state_9
                                                                        (:`NewEnumerator0`
                                                                          (switch `int` _options_index_9
                                                                            (:`0`
                                                                              (bind (_state_10 _options_index_10) (`self.adddialogue` "Eclipse Kid" "But what if I don't see the eclipse? " (`|MakeArray` "I'll come get ya" :!type "Text") "/Game/ryan_stuff/Ryan_DialogueStuff/Audio/Eclipse_10.Eclipse_10"))
                                                                              (switch `/Game/ryan_stuff/Ryan_DialogueStuff/Enum_Dialoguestate` _state_10
                                                                                (:`NewEnumerator0`
                                                                                  (switch `int` _options_index_10
                                                                                    (:`0`
                                                                                      (bind (_state_11 _options_index_11) (`self.adddialogue` "Laz" "I'll come get ya as soon as it shows up. That's a promise kid. Get inside now before you get sick. " (`|MakeArray` "Continue" :!type "Text") "/Game/ryan_stuff/Ryan_DialogueStuff/Audio/Eclipse_11.Eclipse_11"))
                                                                                      (switch `/Game/ryan_stuff/Ryan_DialogueStuff/Enum_Dialoguestate` _state_11
                                                                                        (:`NewEnumerator0`
                                                                                          (switch `int` _options_index_11
                                                                                            (:`0`
                                                                                              (bind (_state_12 _options_index_12) (`self.adddialogue` "Eclipse Kid" "Yes sir. See you in a bit then Lazzy!" (`|MakeArray` "Drink" :!type "Text") "/Game/ryan_stuff/Ryan_DialogueStuff/Audio/Eclipse_12.Eclipse_12"))
                                                                                              (switch `/Game/ryan_stuff/Ryan_DialogueStuff/Enum_Dialoguestate` _state_12
                                                                                                (:`NewEnumerator0`
                                                                                                  (switch `int` _options_index_12
                                                                                                    (:`0`
                                                                                                      (bind _state_13 (`self.adddialogue` "Laz" "Lazzy? Where the hell did these kids come up with that? Oh well. No one to bother me now on this misty now rainy eclispeless day. " (`|MakeArray` "continue drinking/end" :!type "Text") "/Game/ryan_stuff/Ryan_DialogueStuff/Audio/Eclipse_13.Eclipse_13"))
                                                                                                      (switch `/Game/ryan_stuff/Ryan_DialogueStuff/Enum_Dialoguestate` _state_13
                                                                                                        (:`NewEnumerator0`
                                                                                                          (`self.setdialoguetreeindex` 0)
                                                                                                          (`self.closeconversation`))))))))))))))))))))))))))))))))))))))))))))))))))))))