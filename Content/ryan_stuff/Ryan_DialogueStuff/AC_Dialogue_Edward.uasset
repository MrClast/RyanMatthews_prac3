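; Dialogue component for Edward, the robotics repairman, holding his branching conversation with Laz, who comes to have an arm fixed.
; The Dialogue function calls the parent, switches on the dialogue tree index, then chains Adddialogue calls that each set speaker, line, player options and sometimes audio.
; Each call's chosen option index selects the next nested line, with some branches sharing later points in the tree.
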(fn `dialogue`
  (bind _array (`|MakeArray` "Figured" :!type "Text"))
  (bind _array_2 (`|MakeArray` "continue" :!type "Text"))
  (bind _array_3 (`|MakeArray` "Continue" :!type "Text"))
  (bind _array_4 (`|MakeArray` "Continue" :!type "Text"))
  (bind _array_5 (`|MakeArray` "Continue" :!type "Text"))
  (bind _array_6 (`|MakeArray` "Continue" :!type "Text"))
  (bind _array_7 (`|MakeArray` "This wont end well for me" :!type "Text"))
  (bind _array_8 (`|MakeArray` "Continue" :!type "Text"))
  (bind _array_9 (`|MakeArray` "Continue" :!type "Text"))
  (bind _array_10 (`|MakeArray` "Tune up" "Run some tests?" "Anything new?" :!type "Text"))
  (bind _array_11 (`|MakeArray` "Continue" :!type "Text"))
  (bind _array_12 (`|MakeArray` "continue" :!type "Text"))
  (`parent.dialogue`)
  (switch `int` (`self.dialoguetreeindex`)
    (:`0`
      (bind (_state _options_index) (`self.adddialogue` "Laz" "Uhh…hello? Anyone here? " (`|MakeArray` "Continue" :!type "Text") "/Engine/VREditor/Sounds/VR_teleport.VR_teleport"))
      (switch `/Game/ryan_stuff/Ryan_DialogueStuff/Enum_Dialoguestate` _state
        (:`NewEnumerator0`
          (switch `int` _options_index
            (:`0`
              (bind (_state_2 _options_index_2) (`self.adddialogue` "Laz" "I was informed to come to this room to get my arm fixed…" (`|MakeArray` "wrong place?" "I can hear you" :!type "Text")))
              (switch `/Game/ryan_stuff/Ryan_DialogueStuff/Enum_Dialoguestate` _state_2
                (:`NewEnumerator0`
                  (switch `int` _options_index_2
                    (:`0`
                      (bind (_state_3 _options_index_3) (`self.adddialogue` "Laz" "Guess I’m in the wrong place, I’ll be leaving now. " _array_4))
                      (switch `/Game/ryan_stuff/Ryan_DialogueStuff/Enum_Dialoguestate` _state_3
                        (:`NewEnumerator0`
                          (switch `int` _options_index_3
                            (:`0`
                              (bind (_state_4 _options_index_4) (`self.adddialogue` "Edward" "No! Don’t go! Just sit in the chair!" _array_7))
                              (switch `/Game/ryan_stuff/Ryan_DialogueStuff/Enum_Dialoguestate` _state_4
                                (:`NewEnumerator0`
                                  (switch `int` _options_index_4
                                    (:`0`
                                      _)))))))))
                    (:`1`
                      (bind (_state_5 _options_index_5) (`self.adddialogue` "Laz" "Show yourself, I know there is someone in here. I hear the breathing. " _array_4))
                      (switch `/Game/ryan_stuff/Ryan_DialogueStuff/Enum_Dialoguestate` _state_5
                        (:`NewEnumerator0`
                          (switch `int` _options_index_5
                            (:`0`
                              (bind (_state_6 _options_index_6) (`self.adddialogue` "Edward" "Fine you got me….sit in the chair and I’ll come out. " _array_7))
                              (switch `/Game/ryan_stuff/Ryan_DialogueStuff/Enum_Dialoguestate` _state_6
                                (:`NewEnumerator0`
                                  (switch `int` _options_index_6
                                    (:`0`
                                      _))))))))))
                  (bind (_state_7 _options_index_7) (`self.adddialogue` "Laz" "Sitting in the chair is not going to end up well for me is it?" (`|MakeArray` "Continue" :!type "Text")))
                  (switch `/Game/ryan_stuff/Ryan_DialogueStuff/Enum_Dialoguestate` _state_7
                    (:`NewEnumerator0`
                      (switch `int` _options_index_7
                        (:`0`
                          (bind (_state_8 _options_index_8) (`self.adddialogue` "Edward" "No you’ll be perfectly fine. All it will allow me to do is run all the diagnostics I need to. " (`|MakeArray` "Right..." :!type "Text")))
                          (switch `/Game/ryan_stuff/Ryan_DialogueStuff/Enum_Dialoguestate` _state_8
                            (:`NewEnumerator0`
                              (switch `int` _options_index_8
                                (:`0`
                                  (bind (_state_9 _options_index_9) (`self.adddialogue` "Laz" "Right…and if I don’t sit down? " (`|MakeArray` "Continue" :!type "Text")))
                                  (switch `/Game/ryan_stuff/Ryan_DialogueStuff/Enum_Dialoguestate` _state_9
                                    (:`NewEnumerator0`
                                      (switch `int` _options_index_9
                                        (:`0`
                                          (bind (_state_10 _options_index_10) (`self.adddialogue` "Edward" "No other person here can fix that complex machinery on your body. I am all you have friend. " (`|MakeArray` "Great point" :!type "Text")))
                                          (switch `/Game/ryan_stuff/Ryan_DialogueStuff/Enum_Dialoguestate` _state_10
                                            (:`NewEnumerator0`
                                              (switch `int` _options_index_10
                                                (:`0`
                                                  (bind (_state_11 _options_index_11) (`self.adddialogue` "Laz" "You know…you provide a great point however." (`|MakeArray` "Somone else can help" "Stop being weird " :!type "Text")))
                                                  (switch `/Game/ryan_stuff/Ryan_DialogueStuff/Enum_Dialoguestate` _state_11
                                                    (:`NewEnumerator0`
                                                      (switch `int` _options_index_11
                                                        (:`0`
                                                          (bind (_state_12 _options_index_12) (`self.adddialogue` "Laz" "I am sure someone here will be able to figure out everything you know. " _array_12))
                                                          (switch `/Game/ryan_stuff/Ryan_DialogueStuff/Enum_Dialoguestate` _state_12
                                                            (:`NewEnumerator0`
                                                              (switch `int` _options_index_12
                                                                (:`0`
                                                                  (bind (_state_13 _options_index_13) (`self.adddialogue` "Edward" "Meaningless threats! I am the most intelligent here! " (`|MakeArray` "Serious" :!type "Text")))
                                                                  (switch `/Game/ryan_stuff/Ryan_DialogueStuff/Enum_Dialoguestate` _state_13
                                                                    (:`NewEnumerator0`
                                                                      (switch `int` _options_index_13
                                                                        (:`0`
                                                                          (bind (_state_14 _options_index_14) (`self.adddialogue` "Laz" "It's not meaningless, I am being serious. Someone here is smarter than you. And I’ll find them. " (`|MakeArray` "Continue" :!type "Text")))
                                                                          (switch `/Game/ryan_stuff/Ryan_DialogueStuff/Enum_Dialoguestate` _state_14
                                                                            (:`NewEnumerator0`
                                                                              (switch `int` _options_index_14
                                                                                (:`0`
                                                                                  (bind (_state_15 _options_index_15) (`self.adddialogue` "Edward" "Damn you! Fine I’ll come out no need for the chair yet. " _array))
                                                                                  (switch `/Game/ryan_stuff/Ryan_DialogueStuff/Enum_Dialoguestate` _state_15
                                                                                    (:`NewEnumerator0`
                                                                                      (switch `int` _options_index_15
                                                                                        (:`0`
                                                                                          _)))))))))))))))))
                                                        (:`1`
                                                          (bind (_state_16 _options_index_16) (`self.adddialogue` "Laz" "If you don’t stop being weird you won’t understand what makes my body work so well with machinery. " _array_12))
                                                          (switch `/Game/ryan_stuff/Ryan_DialogueStuff/Enum_Dialoguestate` _state_16
                                                            (:`NewEnumerator0`
                                                              (switch `int` _options_index_16
                                                                (:`0`
                                                                  (bind (_state_17 _options_index_17) (`self.adddialogue` "Edward" "Wait. I want to know. I will come out. No need for the chair yet. " _array))
                                                                  (switch `/Game/ryan_stuff/Ryan_DialogueStuff/Enum_Dialoguestate` _state_17
                                                                    (:`NewEnumerator0`
                                                                      (switch `int` _options_index_17
                                                                        (:`0`
                                                                          _))))))))))
                                                      (bind (_state_18 _options_index_18) (`self.adddialogue` "Laz" "Figured you’d eventually see things my way. " (`|MakeArray` "Continue" :!type "Text")))
                                                      (switch `/Game/ryan_stuff/Ryan_DialogueStuff/Enum_Dialoguestate` _state_18
                                                        (:`NewEnumerator0`
                                                          (switch `int` _options_index_18
                                                            (:`0`
                                                              (bind (_state_19 _options_index_19) (`self.adddialogue` "Edward" "You are new here…what is your designation? " (`|MakeArray` "Designation? " :!type "Text")))
                                                              (switch `/Game/ryan_stuff/Ryan_DialogueStuff/Enum_Dialoguestate` _state_19
                                                                (:`NewEnumerator0`
                                                                  (switch `int` _options_index_19
                                                                    (:`0`
                                                                      (bind (_state_20 _options_index_20) (`self.adddialogue` "Laz" "Designation? What are you a computer? " (`|MakeArray` "continue" :!type "Text")))
                                                                      (switch `/Game/ryan_stuff/Ryan_DialogueStuff/Enum_Dialoguestate` _state_20
                                                                        (:`NewEnumerator0`
                                                                          (switch `int` _options_index_20
                                                                            (:`0`
                                                                              (bind (_state_21 _options_index_21) (`self.adddialogue` "Edward" "Computers are my best friend. I tend to speak like them. I meant your name." (`|MakeArray` "Unkillable" "Human wannabe" :!type "Text")))
                                                                              (switch `/Game/ryan_stuff/Ryan_DialogueStuff/Enum_Dialoguestate` _state_21
                                                                                (:`NewEnumerator0`
                                                                                  (switch `int` _options_index_21
                                                                                    (:`0`
                                                                                      (bind (_state_22 _options_index_22) (`self.adddialogue` "Laz" "Lazarus the Unkillable. And you are? " _array_2))
                                                                                      (switch `/Game/ryan_stuff/Ryan_DialogueStuff/Enum_Dialoguestate` _state_22
                                                                                        (:`NewEnumerator0`
                                                                                          (switch `int` _options_index_22
                                                                                            (:`0`
                                                                                              (bind (_state_23 _options_index_23) (`self.adddialogue` "Edward" "Unkillable! Maybe…but certainly not immune to bodily harm. " _array_3))
                                                                                              (switch `/Game/ryan_stuff/Ryan_DialogueStuff/Enum_Dialoguestate` _state_23
                                                                                                (:`NewEnumerator0`
                                                                                                  (switch `int` _options_index_23
                                                                                                    (:`0`
                                                                                                      _)))))))))
                                                                                    (:`1`
                                                                                      (bind (_state_24 _options_index_24) (`self.adddialogue` "Laz" "Laz human wannabe, you are? " _array_2))
                                                                                      (switch `/Game/ryan_stuff/Ryan_DialogueStuff/Enum_Dialoguestate` _state_24
                                                                                        (:`NewEnumerator0`
                                                                                          (switch `int` _options_index_24
                                                                                            (:`0`
                                                                                              (bind (_state_25 _options_index_25) (`self.adddialogue` "Edward" "Human wannabe huh? You and I both. " _array_3))
                                                                                              (switch `/Game/ryan_stuff/Ryan_DialogueStuff/Enum_Dialoguestate` _state_25
                                                                                                (:`NewEnumerator0`
                                                                                                  (switch `int` _options_index_25
                                                                                                    (:`0`
                                                                                                      _))))))))))
                                                                                  (bind (_state_26 _options_index_26) (`self.adddialogue` "Edward" "Oh my name is Edward. I specialize in robotics, but lately have been forced to interact with and repair humans. " (`|MakeArray` "Wording? " :!type "Text")))
                                                                                  (switch `/Game/ryan_stuff/Ryan_DialogueStuff/Enum_Dialoguestate` _state_26
                                                                                    (:`NewEnumerator0`
                                                                                      (switch `int` _options_index_26
                                                                                        (:`0`
                                                                                          (bind (_state_27 _options_index_27) (`self.adddialogue` "Laz" "I really don’t like that wording…what are you implying with repairing humans? " (`|MakeArray` "Continue" :!type "Text")))
                                                                                          (switch `/Game/ryan_stuff/Ryan_DialogueStuff/Enum_Dialoguestate` _state_27
                                                                                            (:`NewEnumerator0`
                                                                                              (switch `int` _options_index_27
                                                                                                (:`0`
                                                                                                  (bind (_state_28 _options_index_28) (`self.adddialogue` "Edward" "Is that not the medical term for it? I repair the parts that are damaged by replacing them with machines. " (`|MakeArray` "Unsure" :!type "Text")))
                                                                                                  (switch `/Game/ryan_stuff/Ryan_DialogueStuff/Enum_Dialoguestate` _state_28
                                                                                                    (:`NewEnumerator0`
                                                                                                      (switch `int` _options_index_28
                                                                                                        (:`0`
                                                                                                          (bind (_state_29 _options_index_29) (`self.adddialogue` "Laz" "I don’t really know enough about the body to argue with that. Just work on the wording a bit. " (`|MakeArray` "Continue" :!type "Text")))
                                                                                                          (switch `/Game/ryan_stuff/Ryan_DialogueStuff/Enum_Dialoguestate` _state_29
                                                                                                            (:`NewEnumerator0`
                                                                                                              (switch `int` _options_index_29
                                                                                                                (:`0`
                                                                                                                  (bind (_state_30 _options_index_30) (`self.adddialogue` "Edward" "Work on the wording? Not following. But anyways, why are you here? " (`|MakeArray` "Arm messing up" "Possble Upgrades" :!type "Text")))
                                                                                                                  (switch `/Game/ryan_stuff/Ryan_DialogueStuff/Enum_Dialoguestate` _state_30
                                                                                                                    (:`NewEnumerator0`
                                                                                                                      (switch `int` _options_index_30
                                                                                                                        (:`0`
                                                                                                                          (bind (_state_31 _options_index_31) (`self.adddialogue` "Laz" "Was told to see you about my arm messing up. " _array_5))
                                                                                                                          (switch `/Game/ryan_stuff/Ryan_DialogueStuff/Enum_Dialoguestate` _state_31
                                                                                                                            (:`NewEnumerator0`
                                                                                                                              (switch `int` _options_index_31
                                                                                                                                (:`0`
                                                                                                                                  (bind (_state_32 _options_index_32) (`self.adddialogue` "Edward" "I can fix that no problem. Just get into the chair and I’ll take a look. " (`|MakeArray` "Fine" :!type "Text")))
                                                                                                                                  (switch `/Game/ryan_stuff/Ryan_DialogueStuff/Enum_Dialoguestate` _state_32
                                                                                                                                    (:`NewEnumerator0`
                                                                                                                                      (switch `int` _options_index_32
                                                                                                                                        (:`0`
                                                                                                                                          (bind (_state_33 _options_index_33) (`self.adddialogue` "Laz" "Fine. I’ll get into the chair this time. " _array_6))
                                                                                                                                          (switch `/Game/ryan_stuff/Ryan_DialogueStuff/Enum_Dialoguestate` _state_33
                                                                                                                                            (:`NewEnumerator0`
                                                                                                                                              (switch `int` _options_index_33
                                                                                                                                                (:`0`
                                                                                                                                                  _)))))))))))))
                                                                                                                        (:`1`
                                                                                                                          (bind (_state_34 _options_index_34) (`self.adddialogue` "Laz" "Was told that you would replace all my fleshy bits and was intrigued. " _array_5))
                                                                                                                          (switch `/Game/ryan_stuff/Ryan_DialogueStuff/Enum_Dialoguestate` _state_34
                                                                                                                            (:`NewEnumerator0`
                                                                                                                              (switch `int` _options_index_34
                                                                                                                                (:`0`
                                                                                                                                  (bind (_state_35 _options_index_35) (`self.adddialogue` "Edward" "OH! Is that really something you want? I could easily make you better than just a man! Get into the chair! " (`|MakeArray` "regret" :!type "Text")))
                                                                                                                                  (switch `/Game/ryan_stuff/Ryan_DialogueStuff/Enum_Dialoguestate` _state_35
                                                                                                                                    (:`NewEnumerator0`
                                                                                                                                      (switch `int` _options_index_35
                                                                                                                                        (:`0`
                                                                                                                                          (bind (_state_36 _options_index_36) (`self.adddialogue` "Laz" "I regret my choice of words. " _array_6))
                                                                                                                                          (switch `/Game/ryan_stuff/Ryan_DialogueStuff/Enum_Dialoguestate` _state_36
                                                                                                                                            (:`NewEnumerator0`
                                                                                                                                              (switch `int` _options_index_36
                                                                                                                                                (:`0`
                                                                                                                                                  _))))))))))))))
                                                                                                                      (bind (_state_37 _options_index_37) (`self.adddialogue` "Edward" "Now that you are in the chair I can take a look at you." (`|MakeArray` "how long" :!type "Text")))
                                                                                                                      (switch `/Game/ryan_stuff/Ryan_DialogueStuff/Enum_Dialoguestate` _state_37
                                                                                                                        (:`NewEnumerator0`
                                                                                                                          (switch `int` _options_index_37
                                                                                                                            (:`0`
                                                                                                                              (bind (_state_38 _options_index_38) (`self.adddialogue` "Laz" "Uhhh…how long is this gonna take? I’ve got places to be man. " (`|MakeArray` "Continue" :!type "Text")))
                                                                                                                              (switch `/Game/ryan_stuff/Ryan_DialogueStuff/Enum_Dialoguestate` _state_38
                                                                                                                                (:`NewEnumerator0`
                                                                                                                                  (switch `int` _options_index_38
                                                                                                                                    (:`0`
                                                                                                                                      (bind (_state_39 _options_index_39) (`self.adddialogue` "Edward" "The Primary check is finished and the arm is working. You can leave whenever you want. " (`|MakeArray` "Great!" :!type "Text")))
                                                                                                                                      (switch `/Game/ryan_stuff/Ryan_DialogueStuff/Enum_Dialoguestate` _state_39
                                                                                                                                        (:`NewEnumerator0`
                                                                                                                                          (switch `int` _options_index_39
                                                                                                                                            (:`0`
                                                                                                                                              (bind (_state_40 _options_index_40) (`self.adddialogue` "Laz" "Oh great then I’m out of here. " (`|MakeArray` "Continue" :!type "Text")))
                                                                                                                                              (switch `/Game/ryan_stuff/Ryan_DialogueStuff/Enum_Dialoguestate` _state_40
                                                                                                                                                (:`NewEnumerator0`
                                                                                                                                                  (switch `int` _options_index_40
                                                                                                                                                    (:`0`
                                                                                                                                                      (bind (_state_41 _options_index_41) (`self.adddialogue` "Edward" "Be warned that when you return, you won't be getting away without an upgrade. " (`|MakeArray` "Inviting" "thanks..." :!type "Text")))
                                                                                                                                                      (switch `/Game/ryan_stuff/Ryan_DialogueStuff/Enum_Dialoguestate` _state_41
                                                                                                                                                        (:`NewEnumerator0`
                                                                                                                                                          (switch `int` _options_index_41
                                                                                                                                                            (:`0`
                                                                                                                                                              (bind (_state_42 _options_index_42) (`self.adddialogue` "Laz" "Gee, how inviting. I really want to come back. " _array_8))
                                                                                                                                                              (switch `/Game/ryan_stuff/Ryan_DialogueStuff/Enum_Dialoguestate` _state_42
                                                                                                                                                                (:`NewEnumerator0`
                                                                                                                                                                  (switch `int` _options_index_42
                                                                                                                                                                    (:`0`
                                                                                                                                                                      _)))))
                                                                                                                                                            (:`1`
                                                                                                                                                              (bind (_state_43 _options_index_43) (`self.adddialogue` "Laz" "Uhh…yeah sure…thanks for the tune up. " _array_8))
                                                                                                                                                              (switch `/Game/ryan_stuff/Ryan_DialogueStuff/Enum_Dialoguestate` _state_43
                                                                                                                                                                (:`NewEnumerator0`
                                                                                                                                                                  (switch `int` _options_index_43
                                                                                                                                                                    (:`0`
                                                                                                                                                                      _))))))
                                                                                                                                                          (bind _state_44 (`self.adddialogue` "Edward" "You’ll be back." (`|MakeArray` "leave" :!type "Text")))
                                                                                                                                                          (switch `/Game/ryan_stuff/Ryan_DialogueStuff/Enum_Dialoguestate` _state_44
                                                                                                                                                            (:`NewEnumerator0`
                                                                                                                                                              (`self.setdialoguetreeindex` 1)
                                                                                                                                                              (`self.closeconversation`))))))))))))))))))))))))))))))))))))))))))))))))))))))))))))))))))))))))))))))
    (:`1`
      (bind (_state_45 _options_index_44) (`self.adddialogue` "Edward" "You returned friend Lazarus!!!" (`|MakeArray` "Yeah, I'm back" "Friend?" :!type "Text")))
      (switch `/Game/ryan_stuff/Ryan_DialogueStuff/Enum_Dialoguestate` _state_45
        (:`NewEnumerator0`
          (switch `int` _options_index_44
            (:`0`
              (bind (_state_46 _options_index_45) (`self.adddialogue` "Laz" "Yeah I guess you were right about me returning pal." _array_9))
              (switch `/Game/ryan_stuff/Ryan_DialogueStuff/Enum_Dialoguestate` _state_46
                (:`NewEnumerator0`
                  (switch `int` _options_index_45
                    (:`0`
                      (bind (_state_47 _options_index_46) (`self.adddialogue` "Edward" "What brings my friend back?" _array_10))
                      (switch `/Game/ryan_stuff/Ryan_DialogueStuff/Enum_Dialoguestate` _state_47
                        (:`NewEnumerator0`
                          (switch `int` _options_index_46
                            (:`0`
                              (bind (_state_48 _options_index_47) (`self.adddialogue` "Laz" "Tune up on the arm" _array_11 :!label _label))
                              (switch `/Game/ryan_stuff/Ryan_DialogueStuff/Enum_Dialoguestate` _state_48
                                (:`NewEnumerator0`
                                  (switch `int` _options_index_47
                                    (:`0`
                                      (bind _state_49 (`self.adddialogue` "Edward" "Get in the chair then friend! " (`|MakeArray` "End" :!type "Text")))
                                      (switch `/Game/ryan_stuff/Ryan_DialogueStuff/Enum_Dialoguestate` _state_49
                                        (:`NewEnumerator0`
                                          (`self.setdialoguetreeindex` 1)
                                          (`self.closeconversation`))))))))
                            (:`1`
                              (bind (_state_50 _options_index_48) (`self.adddialogue` "Laz" "Figured I’d let you test on me for a bit." _array_11 :!label _label_2))
                              (switch `/Game/ryan_stuff/Ryan_DialogueStuff/Enum_Dialoguestate` _state_50
                                (:`NewEnumerator0`
                                  (switch `int` _options_index_48
                                    (:`0`
                                      (bind (_state_51 _options_index_49) (`self.adddialogue` "Edward" "Get in the chair and let us talk while I work. " (`|MakeArray` "Alright" :!type "Text")))
                                      (switch `/Game/ryan_stuff/Ryan_DialogueStuff/Enum_Dialoguestate` _state_51
                                        (:`NewEnumerator0`
                                          (switch `int` _options_index_49
                                            (:`0`
                                              (bind (_state_52 _options_index_50) (`self.adddialogue` "Laz" "I'll get up there. Let's see what you can figure out about me. " (`|MakeArray` "Continue" :!type "Text")))
                                              (switch `/Game/ryan_stuff/Ryan_DialogueStuff/Enum_Dialoguestate` _state_52
                                                (:`NewEnumerator0`
                                                  (switch `int` _options_index_50
                                                    (:`0`
                                                      (bind (_state_53 _options_index_51) (`self.adddialogue` "Edward" "(silence)" (`|MakeArray` "Say something" :!type "Text")))
                                                      (switch `/Game/ryan_stuff/Ryan_DialogueStuff/Enum_Dialoguestate` _state_53
                                                        (:`NewEnumerator0`
                                                          (switch `int` _options_index_51
                                                            (:`0`
                                                              (bind (_state_54 _options_index_52) (`self.adddialogue` "Laz" "Your silence is weird, say something." (`|MakeArray` "Continue" :!type "Text")))
                                                              (switch `/Game/ryan_stuff/Ryan_DialogueStuff/Enum_Dialoguestate` _state_54
                                                                (:`NewEnumerator0`
                                                                  (switch `int` _options_index_52
                                                                    (:`0`
                                                                      (bind (_state_55 _options_index_53) (`self.adddialogue` "Edward" "Hmmm…this is weird. I have never seen a body react like this before. " (`|MakeArray` "Weird how?" :!type "Text")))
                                                                      (switch `/Game/ryan_stuff/Ryan_DialogueStuff/Enum_Dialoguestate` _state_55
                                                                        (:`NewEnumerator0`
                                                                          (switch `int` _options_index_53
                                                                            (:`0`
                                                                              (bind (_state_56 _options_index_54) (`self.adddialogue` "Laz" "Weird how? What are you talking about?" (`|MakeArray` "Continue" :!type "Text")))
                                                                              (switch `/Game/ryan_stuff/Ryan_DialogueStuff/Enum_Dialoguestate` _state_56
                                                                                (:`NewEnumerator0`
                                                                                  (switch `int` _options_index_54
                                                                                    (:`0`
                                                                                      (bind (_state_57 _options_index_55) (`self.adddialogue` "Edward" "When I inject pure adrenaline into your system your body starts to heal itself on its own whenever I make a cut. " (`|MakeArray` "That's Normal" :!type "Text")))
                                                                                      (switch `/Game/ryan_stuff/Ryan_DialogueStuff/Enum_Dialoguestate` _state_57
                                                                                        (:`NewEnumerator0`
                                                                                          (switch `int` _options_index_55
                                                                                            (:`0`
                                                                                              (bind (_state_58 _options_index_56) (`self.adddialogue` "Laz" "It’s always been that way." (`|MakeArray` "Continue" :!type "Text")))
                                                                                              (switch `/Game/ryan_stuff/Ryan_DialogueStuff/Enum_Dialoguestate` _state_58
                                                                                                (:`NewEnumerator0`
                                                                                                  (switch `int` _options_index_56
                                                                                                    (:`0`
                                                                                                      (bind (_state_59 _options_index_57) (`self.adddialogue` "Edward" "That’s not the weird part, friend Lazarus. " (`|MakeArray` "Explain" :!type "Text")))
                                                                                                      (switch `/Game/ryan_stuff/Ryan_DialogueStuff/Enum_Dialoguestate` _state_59
                                                                                                        (:`NewEnumerator0`
                                                                                                          (switch `int` _options_index_57
                                                                                                            (:`0`
                                                                                                              (bind (_state_60 _options_index_58) (`self.adddialogue` "Laz" "Then what is the weird part?" (`|MakeArray` "Continue" :!type "Text")))
                                                                                                              (switch `/Game/ryan_stuff/Ryan_DialogueStuff/Enum_Dialoguestate` _state_60
                                                                                                                (:`NewEnumerator0`
                                                                                                                  (switch `int` _options_index_58
                                                                                                                    (:`0`
                                                                                                                      (bind (_state_61 _options_index_59) (`self.adddialogue` "Edward" "The fact that the body should’ve produced adrenaline whenever you lost your arm. " (`|MakeArray` "And? " :!type "Text")))
                                                                                                                      (switch `/Game/ryan_stuff/Ryan_DialogueStuff/Enum_Dialoguestate` _state_61
                                                                                                                        (:`NewEnumerator0`
                                                                                                                          (switch `int` _options_index_59
                                                                                                                            (:`0`
                                                                                                                              (bind (_state_62 _options_index_60) (`self.adddialogue` "Laz" "Yeah…and?" (`|MakeArray` "Continue" :!type "Text")))
                                                                                                                              (switch `/Game/ryan_stuff/Ryan_DialogueStuff/Enum_Dialoguestate` _state_62
                                                                                                                                (:`NewEnumerator0`
                                                                                                                                  (switch `int` _options_index_60
                                                                                                                                    (:`0`
                                                                                                                                      (bind (_state_63 _options_index_61) (`self.adddialogue` "Edward" "It should not be missing in the first place." (`|MakeArray` "huh" :!type "Text")))
                                                                                                                                      (switch `/Game/ryan_stuff/Ryan_DialogueStuff/Enum_Dialoguestate` _state_63
                                                                                                                                        (:`NewEnumerator0`
                                                                                                                                          (switch `int` _options_index_61
                                                                                                                                            (:`0`
                                                                                                                                              (bind (_state_64 _options_index_62) (`self.adddialogue` "Laz" "That’s….that’s a great point." (`|MakeArray` "Continue" :!type "Text")))
                                                                                                                                              (switch `/Game/ryan_stuff/Ryan_DialogueStuff/Enum_Dialoguestate` _state_64
                                                                                                                                                (:`NewEnumerator0`
                                                                                                                                                  (switch `int` _options_index_62
                                                                                                                                                    (:`0`
                                                                                                                                                      (`self.adddialogue` "Edward" "What happened when you lost your arm? It must’ve caused deep psychological damage for it to never come back." (`|MakeArray` "Lost in a fight" :!type "Text")))))))))))))))))))))))))))))))))))))))))))))))))))))))))))))))
                            (:`2`
                              (bind (_state_65 _options_index_63) (`self.adddialogue` "Laz" "What other bodily upgrades do you have?" _array_11 :!label _label_3))
                              (switch `/Game/ryan_stuff/Ryan_DialogueStuff/Enum_Dialoguestate` _state_65
                                (:`NewEnumerator0`
                                  (switch `int` _options_index_63
                                    (:`0`
                                      (bind (_state_66 _options_index_64) (`self.adddialogue` "Edward" "Nothing special at the moment, maybe some other time." (`|MakeArray` "Shame" :!type "Text")))
                                      (switch `/Game/ryan_stuff/Ryan_DialogueStuff/Enum_Dialoguestate` _state_66
                                        (:`NewEnumerator0`
                                          (switch `int` _options_index_64
                                            (:`0`
                                              (bind _state_67 (`self.adddialogue` "Laz" "Damn shame. Maybe next time then. See ya around Ed." (`|MakeArray` "Leave" :!type "Text")))
                                              (switch `/Game/ryan_stuff/Ryan_DialogueStuff/Enum_Dialoguestate` _state_67
                                                (:`NewEnumerator0`
                                                  (`self.setdialoguetreeindex` 1)
                                                  (`self.closeconversation`))))))))))))))))))))
            (:`1`
              (bind (_state_68 _options_index_65) (`self.adddialogue` "Laz" "I never said we were friends. " _array_9))
              (switch `/Game/ryan_stuff/Ryan_DialogueStuff/Enum_Dialoguestate` _state_68
                (:`NewEnumerator0`
                  (switch `int` _options_index_65
                    (:`0`
                      (bind (_state_69 _options_index_66) (`self.adddialogue` "Edward" "Oh..but we are, so what can i help you with? " _array_10))
                      (switch `/Game/ryan_stuff/Ryan_DialogueStuff/Enum_Dialoguestate` _state_69
                        (:`NewEnumerator0`
                          (switch `int` _options_index_66
                            (:`0`
                              (goto _label))
                            (:`1`
                              (goto _label_2))
                            (:`2`
                              (goto _label_3))))))))))))))))