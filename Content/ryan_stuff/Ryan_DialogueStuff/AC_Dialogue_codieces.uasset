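; Branching dialogue component for Codieces, a talking ancient book that converses with Laz about its missing pages, the past and his rivalry with Nostradamus.
; The Dialogue function switches on the dialogue tree index, chaining Adddialogue nodes whose option indices pick each branch, with some branches rejoining shared lines.
; The first tree introduces the book, and its endings either advance the index to the return-visit tree or remove dialogue progress before closing the conversation.
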(fn `dialogue`
  (bind _array (`|MakeArray` "Continue" :!type "Text"))
  (bind _array_2 (`|MakeArray` "Continue" :!type "Text"))
  (bind _array_3 (`|MakeArray` "Continue" :!type "Text"))
  (bind _array_4 (`|MakeArray` "continue" :!type "Text"))
  (bind _array_5 (`|MakeArray` "continue" :!type "Text"))
  (bind _array_6 (`|MakeArray` "Continue" :!type "Text"))
  (bind _array_7 (`|MakeArray` "Continue" :!type "Text"))
  ;[1 1 1] why does it work????
  (`parent.dialogue`)
  (switch `int` (`self.dialoguetreeindex`)
    (:`0`
      ;[1 1 1] Comment
      (bind (_state _options_index) (`self.adddialogue` "Laz" "Hmph nothing more than an old book" (`|MakeArray` "continue" :!type "Text")))
      (switch `/Game/ryan_stuff/Ryan_DialogueStuff/Enum_Dialoguestate` _state
        (:`NewEnumerator0`
          (switch `int` _options_index
            (:`0`
              ;[1 1 1] Comment
              (bind (_state_2 _options_index_2) (`self.adddialogue` "Laz" "Honestly thought this thing was lost when nostradumus took over, bastard destroyed nearly everything I owned. " (`|MakeArray` "continue" :!type "Text")))
              (switch `/Game/ryan_stuff/Ryan_DialogueStuff/Enum_Dialoguestate` _state_2
                (:`NewEnumerator0`
                  (switch `int` _options_index_2
                    (:`0`
                      ;[1 1 1] Comment
                      (bind (_state_3 _options_index_3) (`self.adddialogue` "Codieces" "You rudly take me from where I can watch everything and the first thing you do is claim I was lost? How fitting for the likes of you. " (`|MakeArray` "This is new" :!type "Text")))
                      (switch `/Game/ryan_stuff/Ryan_DialogueStuff/Enum_Dialoguestate` _state_3
                        (:`NewEnumerator0`
                          (switch `int` _options_index_3
                            (:`0`
                              (bind (_state_4 _options_index_4) (`self.adddialogue` "Laz" "This is new. You were never able to talk before. What is happening here? " (`|MakeArray` "continue" :!type "Text")))
                              (switch `/Game/ryan_stuff/Ryan_DialogueStuff/Enum_Dialoguestate` _state_4
                                (:`NewEnumerator0`
                                  (switch `int` _options_index_4
                                    (:`Default`
                                      (bind (_state_5 _options_index_5) (`self.adddialogue` "Codieces" "I've always been able to speak you ignorant fool! I just chose not to, you were always an annoying child, much like the rest of your pitiful race. You are lucky to even be alive. " (`|MakeArray` "Annoying" "Lucky" :!type "Text")))
                                      (switch `/Game/ryan_stuff/Ryan_DialogueStuff/Enum_Dialoguestate` _state_5
                                        (:`NewEnumerator0`
                                          (switch `int` _options_index_5
                                            (:`0`
                                              (bind (_state_6 _options_index_6) (`self.adddialogue` "Laz" "I don't think i was annoying." (`|MakeArray` "continue" :!type "Text")))
                                              (switch `/Game/ryan_stuff/Ryan_DialogueStuff/Enum_Dialoguestate` _state_6
                                                (:`NewEnumerator0`
                                                  (switch `int` _options_index_6
                                                    (:`Default`
                                                      (bind (_state_7 _options_index_7) (`self.adddialogue` "Codieces" "I have seen all, and have an extensice record of it. You were annoying. " (`|MakeArray` "continue" :!type "Text")))
                                                      (switch `/Game/ryan_stuff/Ryan_DialogueStuff/Enum_Dialoguestate` _state_7
                                                        (:`NewEnumerator0`
                                                          (switch `int` _options_index_7
                                                            (:`Default`
                                                              _)))))))))
                                            (:`1`
                                              (bind (_state_8 _options_index_8) (`self.adddialogue` "Laz" "Luck has noting to do with my current state." (`|MakeArray` "continue" :!type "Text")))
                                              (switch `/Game/ryan_stuff/Ryan_DialogueStuff/Enum_Dialoguestate` _state_8
                                                (:`NewEnumerator0`
                                                  (switch `int` _options_index_8
                                                    (:`Default`
                                                      (bind (_state_9 _options_index_9) (`self.adddialogue` "Codieces" "Lucky doesn't begin to descirbe it. With how much you died that day you shouldn't be walking. " (`|MakeArray` "Continue" :!type "Text")))
                                                      (switch `/Game/ryan_stuff/Ryan_DialogueStuff/Enum_Dialoguestate` _state_9
                                                        (:`NewEnumerator0`
                                                          (switch `int` _options_index_9
                                                            (:`Default`
                                                              _))))))))))
                                          (bind (_state_10 _options_index_10) (`self.adddialogue` "Codieces" "Anyways how did you get a hold of me? Surely I must've been kept in a secure place due to my value? " (`|MakeArray` "lie" "truth" :!type "Text")))
                                          (switch `/Game/ryan_stuff/Ryan_DialogueStuff/Enum_Dialoguestate` _state_10
                                            (:`NewEnumerator0`
                                              (switch `int` _options_index_10
                                                (:`0`
                                                  (bind (_state_11 _options_index_11) (`self.adddialogue` "Laz" "Uhhh...you were kept in a safe place, I just had an easy time getting in. " _array))
                                                  (switch `/Game/ryan_stuff/Ryan_DialogueStuff/Enum_Dialoguestate` _state_11
                                                    (:`NewEnumerator0`
                                                      (switch `int` _options_index_11
                                                        (:`0`
                                                          (bind (_state_12 _options_index_12) (`self.adddialogue` "Codieces" "So you defiled a secure place for little 'ol me? How thoughtful...Anyways I must thank you. I am here to help as best I can. " _array_2))
                                                          (switch `/Game/ryan_stuff/Ryan_DialogueStuff/Enum_Dialoguestate` _state_12
                                                            (:`NewEnumerator0`
                                                              (switch `int` _options_index_12
                                                                (:`0`
                                                                  _)))))))))
                                                (:`1`
                                                  (bind (_state_13 _options_index_13) (`self.adddialogue` "Laz" "Uhhh..You were being kept in the pocket of a once dead Ashen. Dead again now. " _array))
                                                  (switch `/Game/ryan_stuff/Ryan_DialogueStuff/Enum_Dialoguestate` _state_13
                                                    (:`NewEnumerator0`
                                                      (switch `int` _options_index_13
                                                        (:`Default`
                                                          (bind (_state_14 _options_index_14) (`self.adddialogue` "Codieces" "That can't be it....no. I am an acient artifact made by the gods of fire themselves! I could not have just been in someone's pocket! No matter, I must repay my debt as a thank you. " _array_2))
                                                          (switch `/Game/ryan_stuff/Ryan_DialogueStuff/Enum_Dialoguestate` _state_14
                                                            (:`NewEnumerator0`
                                                              (switch `int` _options_index_14
                                                                (:`0`
                                                                  _))))))))))
                                              (bind (_state_15 _options_index_15) (`self.adddialogue` "Laz" "I appreciate the offer for help, I might have to tak you up on that. Say do you still have knowledge from the ancient past?" (`|MakeArray` "continue" :!type "Text")))
                                              (switch `/Game/ryan_stuff/Ryan_DialogueStuff/Enum_Dialoguestate` _state_15
                                                (:`NewEnumerator0`
                                                  (switch `int` _options_index_15
                                                    (:`0`
                                                      (bind (_state_16 _options_index_16) (`self.adddialogue` "Codieces" "I do still have pages, from the past. Although a few appear to be missing. Do you have any ideas where they could be? " (`|MakeArray` "Continue" :!type "Text")))
                                                      (switch `/Game/ryan_stuff/Ryan_DialogueStuff/Enum_Dialoguestate` _state_16
                                                        (:`NewEnumerator0`
                                                          (switch `int` _options_index_16
                                                            (:`0`
                                                              (bind (_state_17 _options_index_17) (`self.adddialogue` "Laz" "Not off the top of my head, no. My guess is random Ashen out in the world have them. " (`|MakeArray` "Continue" :!type "Text")))
                                                              (switch `/Game/ryan_stuff/Ryan_DialogueStuff/Enum_Dialoguestate` _state_17
                                                                (:`NewEnumerator0`
                                                                  (switch `int` _options_index_17
                                                                    (:`0`
                                                                      (bind (_state_18 _options_index_18) (`self.adddialogue` "Codieces" "Do...you think you could bring any back if you find them? " (`|MakeArray` "yes" "no" :!type "Text")))
                                                                      (switch `/Game/ryan_stuff/Ryan_DialogueStuff/Enum_Dialoguestate` _state_18
                                                                        (:`NewEnumerator0`
                                                                          (switch `int` _options_index_18
                                                                            (:`0`
                                                                              (bind (_state_19 _options_index_19) (`self.adddialogue` "Laz" "Yeah, no problem. Just another thing to add to my plate. " (`|MakeArray` "Continue" :!type "Text")))
                                                                              (switch `/Game/ryan_stuff/Ryan_DialogueStuff/Enum_Dialoguestate` _state_19
                                                                                (:`NewEnumerator0`
                                                                                  (switch `int` _options_index_19
                                                                                    (:`0`
                                                                                      (bind _state_20 (`self.adddialogue` "Codieces" "You are a patron saint. Thank you Lazarus, son of the anvil." (`|MakeArray` "continue" :!type "Text")))
                                                                                      (switch `/Game/ryan_stuff/Ryan_DialogueStuff/Enum_Dialoguestate` _state_20
                                                                                        (:`NewEnumerator0`
                                                                                          (`self.setdialoguetreeindex` 1)
                                                                                          (`self.closeconversation`))))))))
                                                                            (:`1`
                                                                              (bind (_state_21 _options_index_20) (`self.adddialogue` "Laz" "No, I don't need to add another thing onto my plate. " (`|MakeArray` "Continue" :!type "Text")))
                                                                              (switch `/Game/ryan_stuff/Ryan_DialogueStuff/Enum_Dialoguestate` _state_21
                                                                                (:`NewEnumerator0`
                                                                                  (switch `int` _options_index_20
                                                                                    (:`0`
                                                                                      (bind (_state_22 _options_index_21) (`self.adddialogue` "Codieces" "It appears you will never change Lazarus. One day you will decide to help me. " (`|MakeArray` "see ya" "changed mind" :!type "Text")))
                                                                                      (switch `/Game/ryan_stuff/Ryan_DialogueStuff/Enum_Dialoguestate` _state_22
                                                                                        (:`NewEnumerator0`
                                                                                          (switch `int` _options_index_21
                                                                                            (:`0`
                                                                                              (bind _state_23 (`self.adddialogue` "Laz" "You'll be stuck as is for now. See ya! " _array_3))
                                                                                              (switch `/Game/ryan_stuff/Ryan_DialogueStuff/Enum_Dialoguestate` _state_23
                                                                                                (:`NewEnumerator0`
                                                                                                  (`self.removedialogueprogress` 5)
                                                                                                  (`self.closeconversation`))))
                                                                                            (:`1`
                                                                                              (bind (_state_24 _options_index_22) (`self.adddialogue` "Laz" "Wait...I've changed my mind. I'll bring any pages I find. " _array_3))
                                                                                              (switch `/Game/ryan_stuff/Ryan_DialogueStuff/Enum_Dialoguestate` _state_24
                                                                                                (:`NewEnumerator0`
                                                                                                  (switch `int` _options_index_22
                                                                                                    (:`0`
                                                                                                      (bind _state_25 (`self.adddialogue` "Codieces" "I knew you weren't all incompentent. I suppose I am more willing to help now. Leave me for the moment, and return later. " (`|MakeArray` "continue" :!type "Text")))
                                                                                                      (switch `/Game/ryan_stuff/Ryan_DialogueStuff/Enum_Dialoguestate` _state_25
                                                                                                        (:`NewEnumerator0`
                                                                                                          (`self.setdialoguetreeindex` 1)
                                                                                                          (`self.closeconversation`))))))))))))))))))))))))))))))))))))))))))))))))))))
    (:`1`
      (bind (_state_26 _options_index_23) (`self.adddialogue` "Codieces" "Welcome back! What can I do for you today my friend? Perhaps a chat? Telling of old stories? Or better yet do you have any pages on you? " (`|MakeArray` "Chat" "pages" "ancient tales" :!type "Text")))
      (switch `/Game/ryan_stuff/Ryan_DialogueStuff/Enum_Dialoguestate` _state_26
        (:`NewEnumerator0`
          (switch `int` _options_index_23
            (:`0`
              (bind (_state_27 _options_index_24) (`self.adddialogue` "Laz" "Just coming along for a chat, How are you holding up in the new home? " _array_4))
              (switch `/Game/ryan_stuff/Ryan_DialogueStuff/Enum_Dialoguestate` _state_27
                (:`NewEnumerator0`
                  (switch `int` _options_index_24
                    (:`0`
                      (bind (_state_28 _options_index_25) (`self.adddialogue` "Codieces" "A chat is something I can handle. I'm holding up fine. Are you feeling okay lad? " (`|MakeArray` "just fine" "could be better" :!type "Text")))
                      (switch `/Game/ryan_stuff/Ryan_DialogueStuff/Enum_Dialoguestate` _state_28
                        (:`NewEnumerator0`
                          (switch `int` _options_index_25
                            (:`0`
                              (bind (_state_29 _options_index_26) (`self.adddialogue` "Laz" "Holding up decently well. The arm is still something I will never be used to honestly." _array_5))
                              (switch `/Game/ryan_stuff/Ryan_DialogueStuff/Enum_Dialoguestate` _state_29
                                (:`NewEnumerator0`
                                  (switch `int` _options_index_26
                                    (:`0`
                                      _)))))
                            (:`1`
                              (bind (_state_30 _options_index_27) (`self.adddialogue` "Laz" "Could be better, I think the arm is still giving me more trouble than necesssary though. " _array_5))
                              (switch `/Game/ryan_stuff/Ryan_DialogueStuff/Enum_Dialoguestate` _state_30
                                (:`NewEnumerator0`
                                  (switch `int` _options_index_27
                                    (:`0`
                                      _))))))
                          (bind (_state_31 _options_index_28) (`self.adddialogue` "Codieces" "The arm huh? It's not very fleshy. I guess some injuries never heal properly huh? Nostradamus is quite the heavy hitter in a fight. " (`|MakeArray` "sure" "not for long" :!type "Text")))
                          (switch `/Game/ryan_stuff/Ryan_DialogueStuff/Enum_Dialoguestate` _state_31
                            (:`NewEnumerator0`
                              (switch `int` _options_index_28
                                (:`0`
                                  (bind (_state_32 _options_index_29) (`self.adddialogue` "Laz" "Sure is. Always has been. But I wouldn't say hes stronger than me. " _array_6))
                                  (switch `/Game/ryan_stuff/Ryan_DialogueStuff/Enum_Dialoguestate` _state_32
                                    (:`NewEnumerator0`
                                      (switch `int` _options_index_29
                                        (:`0`
                                          _)))))
                                (:`1`
                                  (bind (_state_33 _options_index_30) (`self.adddialogue` "Laz" "Not for much longer, I've always been close to him. He jsut got the upper hand last time.  " _array_6))
                                  (switch `/Game/ryan_stuff/Ryan_DialogueStuff/Enum_Dialoguestate` _state_33
                                    (:`NewEnumerator0`
                                      (switch `int` _options_index_30
                                        (:`0`
                                          _))))))
                              (bind (_state_34 _options_index_31) (`self.adddialogue` "Codieces" "He leads them for a reason, If you were stronger than him from the start we wouldn’t be here. " (`|MakeArray` "HUH?" :!type "Text")))
                              (switch `/Game/ryan_stuff/Ryan_DialogueStuff/Enum_Dialoguestate` _state_34
                                (:`NewEnumerator0`
                                  (switch `int` _options_index_31
                                    (:`0`
                                      (bind (_state_35 _options_index_32) (`self.adddialogue` "Laz" "Huh? What are you implying by that? I mean he’s strong but not that much stronger than me. I would say he’s kind of in the area of being more skilled. Pure strength has nothing to do with it. " (`|MakeArray` "Continue" :!type "Text")))
                                      (switch `/Game/ryan_stuff/Ryan_DialogueStuff/Enum_Dialoguestate` _state_35
                                        (:`NewEnumerator0`
                                          (switch `int` _options_index_32
                                            (:`0`
                                              (bind (_state_36 _options_index_33) (`self.adddialogue` "Codieces" "More skilled you say? Well surely that won’t last much longer, you seem to be improving at an incredible rate from everything I’ve seen at least. " (`|MakeArray` "Tech" :!type "Text")))
                                              (switch `/Game/ryan_stuff/Ryan_DialogueStuff/Enum_Dialoguestate` _state_36
                                                (:`NewEnumerator0`
                                                  (switch `int` _options_index_33
                                                    (:`0`
                                                      (bind (_state_37 _options_index_34) (`self.adddialogue` "Laz" "Hasn’t been pure physical improvement alone. I seem to be finding myself relying on technology more and more. " (`|MakeArray` "continue" :!type "Text")))
                                                      (switch `/Game/ryan_stuff/Ryan_DialogueStuff/Enum_Dialoguestate` _state_37
                                                        (:`NewEnumerator0`
                                                          (switch `int` _options_index_34
                                                            (:`0`
                                                              (bind (_state_38 _options_index_35) (`self.adddialogue` "Codieces" "That’s just you relying upon your resources around you. Nothing wrong with that. If anything I would say it makes you human. " (`|MakeArray` "More human" :!type "Text")))
                                                              (switch `/Game/ryan_stuff/Ryan_DialogueStuff/Enum_Dialoguestate` _state_38
                                                                (:`NewEnumerator0`
                                                                  (switch `int` _options_index_35
                                                                    (:`0`
                                                                      (bind (_state_39 _options_index_36) (`self.adddialogue` "Laz" "Some of the Ashen don’t want to be more like humans. It’s always been seen as a sign of weakness. " (`|MakeArray` "Continue" :!type "Text")))
                                                                      (switch `/Game/ryan_stuff/Ryan_DialogueStuff/Enum_Dialoguestate` _state_39
                                                                        (:`NewEnumerator0`
                                                                          (switch `int` _options_index_36
                                                                            (:`0`
                                                                              (bind (_state_40 _options_index_37) (`self.adddialogue` "Codieces" "Being more human is never a bad thing, humans feel emotions you and I can not dream of feeling. To be human is to fight for something you believe in. To be Human is to be alive." (`|MakeArray` "Silence" :!type "Text")))
                                                                              (switch `/Game/ryan_stuff/Ryan_DialogueStuff/Enum_Dialoguestate` _state_40
                                                                                (:`NewEnumerator0`
                                                                                  (switch `int` _options_index_37
                                                                                    (:`0`
                                                                                      (bind (_state_41 _options_index_38) (`self.adddialogue` "Codieces" "And you are alive aren’t you? " (`|MakeArray` "Suppose so" :!type "Text")))
                                                                                      (switch `/Game/ryan_stuff/Ryan_DialogueStuff/Enum_Dialoguestate` _state_41
                                                                                        (:`NewEnumerator0`
                                                                                          (switch `int` _options_index_38
                                                                                            (:`0`
                                                                                              (bind (_state_42 _options_index_39) (`self.adddialogue` "Laz" "I suppose I am. But is that a good enough reason to keep going down the route I am? " (`|MakeArray` "Continue" :!type "Text")))
                                                                                              (switch `/Game/ryan_stuff/Ryan_DialogueStuff/Enum_Dialoguestate` _state_42
                                                                                                (:`NewEnumerator0`
                                                                                                  (switch `int` _options_index_39
                                                                                                    (:`0`
                                                                                                      (bind (_state_43 _options_index_40) (`self.adddialogue` "Codieces" "Maybe, maybe not. It is not for me to decide.  You must come to that conclusion yourself boy. Some other people wish to talk with you before you head out. So i wont keep you to myself." (`|MakeArray` "Thanks " :!type "Text")))
                                                                                                      (switch `/Game/ryan_stuff/Ryan_DialogueStuff/Enum_Dialoguestate` _state_43
                                                                                                        (:`NewEnumerator0`
                                                                                                          (switch `int` _options_index_40
                                                                                                            (:`0`
                                                                                                              (bind _state_44 (`self.adddialogue` "Laz" "Thank you, and see you later Codieces. And for a book full of knowledge. You can think like a human when needed. " (`|MakeArray` "end" :!type "Text")))
                                                                                                              (switch `/Game/ryan_stuff/Ryan_DialogueStuff/Enum_Dialoguestate` _state_44
                                                                                                                (:`NewEnumerator0`
                                                                                                                  (`self.setdialoguetreeindex` 1)
                                                                                                                  (`self.closeconversation`))))))))))))))))))))))))))))))))))))))))))))))))))))
            (:`1`
              (bind (_state_45 _options_index_41) (`self.adddialogue` "Laz" "I think I have some pages here. I'll let you look at them. " _array_4))
              (switch `/Game/ryan_stuff/Ryan_DialogueStuff/Enum_Dialoguestate` _state_45
                (:`NewEnumerator0`
                  (switch `int` _options_index_41
                    (:`0`
                      (bind (_state_46 _options_index_42) (`self.adddialogue` "Codieces" "Yes let me take a look at them! Bring me enough and I could tell the girl over there how to make a stronger blade for you.  " (`|MakeArray` "Intrige " "Meh" :!type "Text")))
                      (switch `/Game/ryan_stuff/Ryan_DialogueStuff/Enum_Dialoguestate` _state_46
                        (:`NewEnumerator0`
                          (switch `int` _options_index_42
                            (:`0`
                              (bind (_state_47 _options_index_43) (`self.adddialogue` "Laz" "You've peaked my intrest. I'll be sure to bring any and all I find now. " _array_7))
                              (switch `/Game/ryan_stuff/Ryan_DialogueStuff/Enum_Dialoguestate` _state_47
                                (:`NewEnumerator0`
                                  (switch `int` _options_index_43
                                    (:`0`
                                      (bind _state_48 (`self.adddialogue` "Codieces" "So thats what drives you, rewards. Interesting, off with you while I gander these pages. " (`|MakeArray` "end" :!type "Text")))
                                      (switch `/Game/ryan_stuff/Ryan_DialogueStuff/Enum_Dialoguestate` _state_48
                                        (:`NewEnumerator0`
                                          (`self.setdialoguetreeindex` 1)
                                          (`self.closeconversation`))))))))
                            (:`1`
                              (bind (_state_49 _options_index_44) (`self.adddialogue` "Laz" "Meh, just a cool bonus on top of it all honestly." _array_7))
                              (switch `/Game/ryan_stuff/Ryan_DialogueStuff/Enum_Dialoguestate` _state_49
                                (:`NewEnumerator0`
                                  (switch `int` _options_index_44
                                    (:`0`
                                      (bind _state_50 (`self.adddialogue` "Codieces" "Act a little bit more gratefull next time. Off with you. " (`|MakeArray` "end" :!type "Text")))
                                      (switch `/Game/ryan_stuff/Ryan_DialogueStuff/Enum_Dialoguestate` _state_50
                                        (:`NewEnumerator0`
                                          (`self.setdialoguetreeindex` 1)
                                          (`self.closeconversation`))))))))))))))))
            (:`2`
              (bind (_state_51 _options_index_45) (`self.adddialogue` "Laz" "I'd like to see some of the ancient tales you got in there. " _array_4))
              (switch `/Game/ryan_stuff/Ryan_DialogueStuff/Enum_Dialoguestate` _state_51
                (:`NewEnumerator0`
                  (switch `int` _options_index_45
                    (:`0`
                      (bind _state_52 (`self.adddialogue` "Codieces" "Classic...only used for ancient knowledge. Fine my pages are open to you. " (`|MakeArray` "open codex" :!type "Text")))
                      (switch `/Game/ryan_stuff/Ryan_DialogueStuff/Enum_Dialoguestate` _state_52
                        (:`NewEnumerator0`
                          (`self.setdialoguetreeindex` 1)
                          (`self.closeconversation`)
                          (bind _returnvalue (`|CreateWidget` "/Game/ryan_stuff/widgets/W_Codex.W_Codex_C" (`GameplayStatics.GetPlayerController` 0)))
                          (`UserWidget.AddToViewport` _returnvalue 0))))))))))))))