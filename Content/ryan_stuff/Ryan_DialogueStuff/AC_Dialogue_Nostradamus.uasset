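; Dialogue component that scripts a conversation between Nostradamus and his brother Laz about the repeating day Laz appears to have caused.
; The Dialogue override calls its parent, then chains Adddialogue calls, each supplying speaker, line and usually a single response option.
; Each next line nests under the previous call's Pass Through state and option index, forming a linear exchange that ends on Nostradamus's option-less warning about Andras.
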(fn `dialogue`
  (`parent.dialogue`)
  (bind (_state _options_index) (`self.adddialogue` "Nostradamus" "Oh my dear brother, you must be the cause of this. I can't seem to remember the last time the same day kept repeating itself. " (`|MakeArray` "Not me" :!type "Text")))
  (switch `/Game/ryan_stuff/Ryan_DialogueStuff/Enum_Dialoguestate` _state
    (:`NewEnumerator0`
      (switch `int` _options_index
        (:`0`
          (bind (_state_2 _options_index_2) (`self.adddialogue` "Laz" "You think I want to be stuck in this repeating hell? Also I should kill you now. " (`|MakeArray` "continue" :!type "Text")))
          (switch `/Game/ryan_stuff/Ryan_DialogueStuff/Enum_Dialoguestate` _state_2
            (:`NewEnumerator0`
              (switch `int` _options_index_2
                (:`0`
                  (bind (_state_3 _options_index_3) (`self.adddialogue` "Nostradamus" "If I really wanted to you would be dead by now, but then that would just put us back where we began. With this day repeating itself again and again.  " (`|MakeArray` "Why haven't you" :!type "Text")))
                  (switch `/Game/ryan_stuff/Ryan_DialogueStuff/Enum_Dialoguestate` _state_3
                    (:`NewEnumerator0`
                      (switch `int` _options_index_3
                        (:`0`
                          (bind (_state_4 _options_index_4) (`self.adddialogue` "Laz" "Is that whats going on? This sense of dejavu, is really just a day constantly repeating?" (`|MakeArray` "Continue" :!type "Text")))
                          (switch `/Game/ryan_stuff/Ryan_DialogueStuff/Enum_Dialoguestate` _state_4
                            (:`NewEnumerator0`
                              (switch `int` _options_index_4
                                (:`0`
                                  (bind (_state_5 _options_index_5) (`self.adddialogue` "Nostradamus" "Yes it is little brother, and you appear to be the cause of all of it. You triggered your body's ultimate failsafe. And our making us suffer for it. " (`|MakeArray` "Failsafe?" :!type "Text")))
                                  (switch `/Game/ryan_stuff/Ryan_DialogueStuff/Enum_Dialoguestate` _state_5
                                    (:`NewEnumerator0`
                                      (switch `int` _options_index_5
                                        (:`0`
                                          (bind (_state_6 _options_index_6) (`self.adddialogue` "Laz" "Why am I the cause of this? And you never answered me why are you even here? Aren't we trying to kill each other? " (`|MakeArray` "Continue" :!type "Text")))
                                          (switch `/Game/ryan_stuff/Ryan_DialogueStuff/Enum_Dialoguestate` _state_6
                                            (:`NewEnumerator0`
                                              (switch `int` _options_index_6
                                                (:`0`
                                                  (bind (_state_7 _options_index_7) (`self.adddialogue` "Nostradamus" "You saw something you didn't like and you proceeded to make a never ending day. And all I want to do is help you break out of here so we can kill each other. " (`|MakeArray` "Continue" :!type "Text")))
                                                  (switch `/Game/ryan_stuff/Ryan_DialogueStuff/Enum_Dialoguestate` _state_7
                                                    (:`NewEnumerator0`
                                                      (switch `int` _options_index_7
                                                        (:`0`
                                                          (`self.adddialogue` "Nostradamus" "All I have left to say is this. Stop being afraid of what comes after you defeat Andras. You can't change it. "))))))))))))))))))))))))))))))