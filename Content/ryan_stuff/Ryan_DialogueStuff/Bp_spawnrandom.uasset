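; Spawner actor that randomly places either an old man NPC or a vending machine when play begins.
; BeginPlay passes through a DoOnce, then switches on a random integer to pick one of the two classes with equal odds.
; Each class spawns at the world location of its own component, Oldmanspawn or Vendingspawn.
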(event `self.ReceiveBeginPlay`
  (`/Engine/EditorBlueprintResources/StandardMacros.DoOnce` false
    (:`Completed`
      (switch `int` (`KismetMathLibrary.RandomIntegerInRange` 0 1)
        (:`0`
          (`|SpawnActorFromClass` "/Game/ryan_stuff/Ryan_DialogueStuff/NPC_oldmant.NPC_oldmant_C" (`KismetMathLibrary.Conv_VectorToTransform` (`SceneComponent.K2_GetComponentLocation` (`self.oldmanspawn`))) "Undefined" "MultiplyWithRoot" null null))
        (:`1`
          (`|SpawnActorFromClass` "/Game/ryan_stuff/Ryan_DialogueStuff/BP_vending.BP_vending_C" (`KismetMathLibrary.Conv_VectorToTransform` (`SceneComponent.K2_GetComponentLocation` (`self.vendingspawn`))) "Undefined" "MultiplyWithRoot" null null))))))

(fn `UserConstructionScript`)