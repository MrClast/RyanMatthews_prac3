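; Dialogue component for the Old Man NPC, holding his scripted conversation with Laz, in which he hints at repeated past meetings and is revealed as Joseph.
; It overrides Dialogue, calls the parent, then for tree index 0 runs a linear chain of Adddialogue calls with a single option each.
; Each line advances on Pass Through, and the last closes the conversation.
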(fn `dialogue`
  (`parent.dialogue`)
  (switch `int` (`self.dialoguetreeindex`)
    (:`0`
      (bind (_state _options_index) (`self.adddialogue` "Old Man" "How many times have you done this? " (`|MakeArray` "Confusion" :!type "Text")))
      (switch `/Game/ryan_stuff/Ryan_DialogueStuff/Enum_Dialoguestate` _state
        (:`NewEnumerator0`
          (switch `int` _options_index
            (:`0`
              (bind (_state_2 _options_index_2) (`self.adddialogue` "Laz" "Huh? Have we met before?" (`|MakeArray` "Continue" :!type "Text")))
              (switch `/Game/ryan_stuff/Ryan_DialogueStuff/Enum_Dialoguestate` _state_2
                (:`NewEnumerator0`
                  (switch `int` _options_index_2
                    (:`0`
                      (bind (_state_3 _options_index_3) (`self.adddialogue` "Old Man" "We have met many times over the last 200 years Lazarus. " (`|MakeArray` "Confusion" :!type "Text")))
                      (switch `/Game/ryan_stuff/Ryan_DialogueStuff/Enum_Dialoguestate` _state_3
                        (:`NewEnumerator0`
                          (switch `int` _options_index_3
                            (:`0`
                              (bind (_state_4 _options_index_4) (`self.adddialogue` "Laz" "I never said my name or age. How did you know those things? " (`|MakeArray` "Continue" :!type "Text")))
                              (switch `/Game/ryan_stuff/Ryan_DialogueStuff/Enum_Dialoguestate` _state_4
                                (:`NewEnumerator0`
                                  (switch `int` _options_index_4
                                    (:`0`
                                      (bind (_state_5 _options_index_5) (`self.adddialogue` "Old Man" "Because, we have been in this position before. Many many times. " (`|MakeArray` "continue" :!type "Text")))
                                      (switch `/Game/ryan_stuff/Ryan_DialogueStuff/Enum_Dialoguestate` _state_5
                                        (:`NewEnumerator0`
                                          (switch `int` _options_index_5
                                            (:`0`
                                              (bind (_state_6 _options_index_6) (`self.adddialogue` "Old Man" "The look of confusion on your face never fails to amaze me. You have been here in this same situation so many times. So much that it feels new everytime.  " (`|MakeArray` "But this is new. " :!type "Text")))
                                              (switch `/Game/ryan_stuff/Ryan_DialogueStuff/Enum_Dialoguestate` _state_6
                                                (:`NewEnumerator0`
                                                  (switch `int` _options_index_6
                                                    (:`0`
                                                      (bind (_state_7 _options_index_7) (`self.adddialogue` "Laz" "But this is new. I haven't found Andras at any point. Unless I have and I fail somewhere else down the line. " (`|MakeArray` "Permanent end?" :!type "Text")))
                                                      (switch `/Game/ryan_stuff/Ryan_DialogueStuff/Enum_Dialoguestate` _state_7
                                                        (:`NewEnumerator0`
                                                          (switch `int` _options_index_7
                                                            (:`0`
                                                              (bind (_state_8 _options_index_8) (`self.adddialogue` "Laz" "Do I meet my final end soon? Is that what you are, death personified?" (`|MakeArray` "Continue" :!type "Text")))
                                                              (switch `/Game/ryan_stuff/Ryan_DialogueStuff/Enum_Dialoguestate` _state_8
                                                                (:`NewEnumerator0`
                                                                  (switch `int` _options_index_8
                                                                    (:`0`
                                                                      (bind (_state_9 _options_index_9) (`self.adddialogue` "Old Man" "If I was death it would make everything in life simplier. No I am someone you have already met before.  " (`|MakeArray` "Name?" :!type "Text")))
                                                                      (switch `/Game/ryan_stuff/Ryan_DialogueStuff/Enum_Dialoguestate` _state_9
                                                                        (:`NewEnumerator0`
                                                                          (switch `int` _options_index_9
                                                                            (:`0`
                                                                              (bind (_state_10 _options_index_10) (`self.adddialogue` "Laz" "I don't recall telling any human I've lived for over 200 years. So what is your name then if it isn't death?" (`|MakeArray` "continue" :!type "Text")))
                                                                              (switch `/Game/ryan_stuff/Ryan_DialogueStuff/Enum_Dialoguestate` _state_10
                                                                                (:`NewEnumerator0`
                                                                                  (switch `int` _options_index_10
                                                                                    (:`0`
                                                                                      (bind (_state_11 _options_index_11) (`self.adddialogue` "Old Man" "The fact you cannot remember your original name is quite concerning. Perhaps Joseph is truly no more and I am all that remains of him. " (`|MakeArray` "long dead" :!type "Text")))
                                                                                      (switch `/Game/ryan_stuff/Ryan_DialogueStuff/Enum_Dialoguestate` _state_11
                                                                                        (:`NewEnumerator0`
                                                                                          (switch `int` _options_index_11
                                                                                            (:`0`
                                                                                              (bind (_state_12 _options_index_12) (`self.adddialogue` "Laz" "That name has been long since dead. Joseph died the day Lazarus was born. We are done here. But if we meet again I hope you don't lie about the name." (`|MakeArray` "continue" :!type "Text")))
                                                                                              (switch `/Game/ryan_stuff/Ryan_DialogueStuff/Enum_Dialoguestate` _state_12
                                                                                                (:`NewEnumerator0`
                                                                                                  (switch `int` _options_index_12
                                                                                                    (:`0`
                                                                                                      (bind _state_13 (`self.adddialogue` "Joseph" "Oh, we will meet again. The journey ends shortly after Andras falls. Lazarus, before you go let me ask this. Is what you are doing right? . " (`|MakeArray` "end" :!type "Text")))
                                                                                                      (switch `/Game/ryan_stuff/Ryan_DialogueStuff/Enum_Dialoguestate` _state_13
                                                                                                        (:`NewEnumerator0`
                                                                                                          (`self.closeconversation`))))))))))))))))))))))))))))))))))))))))))))))))))))))