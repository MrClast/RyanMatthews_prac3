(event `self.Box.OnComponentBeginOverlap`
  (params (OverlappedComponent :type "PrimitiveComponent Object Reference") (OtherActor :type "Actor Object Reference") (OtherComp :type "PrimitiveComponent Object Reference") (OtherBodyIndex :type Integer) (bFromSweep :type Boolean) (SweepResult :type "HitResult Structure (by ref)"))
  (if (`self.ActorHasTag` OtherActor "player")
    (bind _asbp_third_person_character (cast `/Game/ThirdPerson/Blueprints/BP_ThirdPersonCharacter` (`GameplayStatics.GetPlayerCharacter` 0)))
    (bind _quipwidget (`/Game/ThirdPerson/Blueprints/BP_ThirdPersonCharacter.quipwidget` _asbp_third_person_character))
    (`UserWidget.AddToViewport` _quipwidget 0)
    (`/Game/ryan_stuff/widgets/W_quip.update quip text` _quipwidget "Thanks, needed the pick me up")
    (`GameplayStatics.PlaySound2D` null 1.0 1.0 0.0 null null)
    (if (< (`/Game/ThirdPerson/Blueprints/BP_ThirdPersonCharacter.health` _asbp_third_person_character) 100.0)
      (set `/Game/ThirdPerson/Blueprints/BP_ThirdPersonCharacter.health` 100.0 _asbp_third_person_character)
      (`KismetSystemLibrary.Delay` 1.0)
      (`Widget.RemoveFromParent` _quipwidget))))

(fn `UserConstructionScript`)