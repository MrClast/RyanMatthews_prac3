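; Base actor component for branching dialogue, which opens a W_Dialogue widget and notifies its owner when the conversation closes.
; Child classes can override the empty Dialogue function, which replays from the start on each progress step.
; AddDialogue returns saved choices from an index-to-option map, or displays the line when none is saved.
; Optional voice audio plays through a runtime-created AudioComponent, async-loading unloaded sounds.
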(event `self.ReceiveBeginPlay`
  (if (`self.UseAudio`)
    (bind _returnvalue (`|AddComponentByClass` :`self` (`self.GetOwner`) :`Class` "/Script/Engine.AudioComponent"))
    (set `self.audiocomponent` _returnvalue)))

(event `load dialogue audio`
  (params (`sound base` :type "SoundBase Soft Object Reference"))
  (bind _object (`|LoadAsset` `sound base`)
    (:`Completed`
      (bind _assound_base (cast `SoundBase` _object))
      (`AudioComponent.SetSound` (`self.audiocomponent`) _assound_base)
      (`AudioComponent.Play` (`self.audiocomponent`) 0.0))))

(fn `adddialogue`
  (params (speaker :type Text) (Dialogue :type Text) (Options :type "Array of Text") (`Dialogue Audio` :type "SoundBase Soft Object Reference"))
  (returns (State :type "/Game/ryan_stuff/Ryan_DialogueStuff/Enum_Dialoguestate Enum") (`Options index` :type Integer))
  (bind (_value _returnvalue) (`BlueprintMapLibrary.Map_Find` (`self.dialogueprogress`) (`self.dialogueindex`)))
  (`/Engine/EditorBlueprintResources/StandardMacros.IncrementInt` (`self.dialogueindex`)
    (:`  `
      (if _returnvalue
        (return "NewEnumerator0" _value)
        (else
          (`/Game/ryan_stuff/widgets/W_Dialogue.UpdateDialogueText` (`self.dialoguewidget`) (`self.dialogueindex`) (`local.speaker`) (`local.Dialogue`) (`local.Options`))
          (`self.PlaydialogueAudio` (`local.Dialogue Audio`))
          (return "NewEnumerator1" 0))))))

(fn `cleardialogueprogress`
  (`BlueprintMapLibrary.Map_Clear` (`self.dialogueprogress`)))

(fn `closeconversation`
  (`Widget.RemoveFromParent` (`self.dialoguewidget`))
  (message `/Game/ryan_stuff/Ryan_DialogueStuff/BPI_Interactable.ConversationCLosed` (`self.GetOwner`)))

(fn `dialogue`)

(fn `openconversation`
  (bind _returnvalue (`|CreateWidget` "/Game/ryan_stuff/widgets/W_Dialogue.W_Dialogue_C" null self))
  (bind _output_get (set `self.dialoguewidget` _returnvalue))
  (`UserWidget.AddToViewport` _output_get 0)
  (`self.progressdialogue`))

(fn `PlaydialogueAudio`
  (params (audio :type "SoundBase Soft Object Reference (by ref)"))
  (bind _audio (`local.audio`))
  (bind _output (`|ConvertAsset` _audio))
  (if (and (`KismetSystemLibrary.IsValidSoftObjectReference` audio) (`self.UseAudio`))
    (`/Engine/EditorBlueprintResources/StandardMacros.IsValid` _output
      (:`Is Valid`
        (`AudioComponent.SetSound` (`self.audiocomponent`) _output)
        (`AudioComponent.Play` (`self.audiocomponent`) 0.0))
      (:`Is Not Valid`
        (`self.load dialogue audio` _audio)))))

(fn `progressdialogue`
  (set `self.dialogueindex` -1)
  (`self.dialogue`))

(fn `removedialogueprogress`
  (params (`Progress Steps` :type Integer))
  (for _index (range (+ `Progress Steps` 1))
    (`BlueprintMapLibrary.Map_Remove` (`self.dialogueprogress`) (- (`self.dialogueindex`) _index))))

(fn `setdialoguetreeindex`
  (params (`Dialogue Tree Index` :type Integer))
  (set `self.dialoguetreeindex` `Dialogue Tree Index`)
  (`self.cleardialogueprogress`))

(fn `updateselectedoption`
  (params (`Progress Index` :type "Integer (by ref)") (`Option index` :type "Integer (by ref)"))
  (`BlueprintMapLibrary.Map_Add` (`self.dialogueprogress`) `Progress Index` `Option index`)
  (`self.progressdialogue`))