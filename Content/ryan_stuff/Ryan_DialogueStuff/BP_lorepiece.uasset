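; BP_lorepiece is a lore pickup actor that shows the player a random piece of lore text when touched.
; BeginPlay creates a W_lore widget and stores it as Lorescreen.
; When an actor tagged "player" overlaps its Box, it adds the widget to the viewport, passes a random Loretext entry to Updatetext, then destroys itself.
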(event `self.ReceiveBeginPlay`
  (bind _returnvalue (`|CreateWidget` "/Game/ryan_stuff/widgets/W_lore.W_lore_C"))
  (set `self.lorescreen` _returnvalue))

(event `self.Box.OnComponentBeginOverlap`
  (params (OverlappedComponent :type "PrimitiveComponent Object Reference") (OtherActor :type "Actor Object Reference") (OtherComp :type "PrimitiveComponent Object Reference") (OtherBodyIndex :type Integer) (bFromSweep :type Boolean) (SweepResult :type "HitResult Structure (by ref)"))
  (bind _lorescreen (`self.lorescreen`))
  (bind _loretext (`self.loretext`))
  (if (`self.ActorHasTag` OtherActor "player")
    (`UserWidget.AddToViewport` _lorescreen 0)
    (`/Game/ryan_stuff/widgets/W_lore.updatetext` _lorescreen (`|GetArrayItem` _loretext (`KismetMathLibrary.RandomIntegerInRange` 0 (- (`KismetArrayLibrary.Array_Length` _loretext) 1))))
    (`self.K2_DestroyActor`)))

(fn `UserConstructionScript`)