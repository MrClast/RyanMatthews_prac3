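; Dialogue component holding Stevens's scripted conversation with Laz (Lazarus), who is sent to stop Andras at a decaying lab to the west.
; It overrides Dialogue, calls the parent, then runs a linear chain of Adddialogue calls alternating between the two speakers.
; Each line offers a single option, and its Pass Through state with that option selected leads to the next, until Closeconversation ends it.
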(fn `dialogue`
  (`parent.dialogue`)
  (bind (_state _options_index) (`self.adddialogue` "Stevens" "WHAT THE HELL ARE YOU STILL DOING HERE?" (`|MakeArray` "stop yelling" :!type "Text")))
  (switch `/Game/ryan_stuff/Ryan_DialogueStuff/Enum_Dialoguestate` _state
    (:`NewEnumerator0`
      (switch `int` _options_index
        (:`0`
          (bind (_state_2 _options_index_2) (`self.adddialogue` "Laz" "Look old man, I'm going to need you to stop yelling at me. " (`|MakeArray` "Continue" :!type "Text")))
          (switch `/Game/ryan_stuff/Ryan_DialogueStuff/Enum_Dialoguestate` _state_2
            (:`NewEnumerator0`
              (switch `int` _options_index_2
                (:`0`
                  (bind (_state_3 _options_index_3) (`self.adddialogue` "Stevens" "You said ages ago you were here to help humanity! You have not done anything worth while since you got here! " (`|MakeArray` "Done plenty" :!type "Text")))
                  (switch `/Game/ryan_stuff/Ryan_DialogueStuff/Enum_Dialoguestate` _state_3
                    (:`NewEnumerator0`
                      (switch `int` _options_index_3
                        (:`0`
                          (bind (_state_4 _options_index_4) (`self.adddialogue` "Laz" "I have done plenty around here Stevens. But what would you like me to do if I need to pull my weight a little bit more?" (`|MakeArray` "Continue" :!type "Text")))
                          (switch `/Game/ryan_stuff/Ryan_DialogueStuff/Enum_Dialoguestate` _state_4
                            (:`NewEnumerator0`
                              (switch `int` _options_index_4
                                (:`0`
                                  (bind (_state_5 _options_index_5) (`self.adddialogue` "Stevens" "We have gotten word that an old pal of yours, Andras has built himself a device that allows the user to summon the armies of the dead." (`|MakeArray` "Odd" :!type "Text")))
                                  (switch `/Game/ryan_stuff/Ryan_DialogueStuff/Enum_Dialoguestate` _state_5
                                    (:`NewEnumerator0`
                                      (switch `int` _options_index_5
                                        (:`0`
                                          (bind (_state_6 _options_index_6) (`self.adddialogue` "Laz" "Well thats odd. Why would that old man try to give himself the same power my brother has?" (`|MakeArray` "Continue" :!type "Text")))
                                          (switch `/Game/ryan_stuff/Ryan_DialogueStuff/Enum_Dialoguestate` _state_6
                                            (:`NewEnumerator0`
                                              (switch `int` _options_index_6
                                                (:`0`
                                                  (bind (_state_7 _options_index_7) (`self.adddialogue` "Stevens" "Because all of you Ashen are the same. No sense of pride and willing to copy a cheap trick for more power. " (`|MakeArray` "okay then" :!type "Text")))
                                                  (switch `/Game/ryan_stuff/Ryan_DialogueStuff/Enum_Dialoguestate` _state_7
                                                    (:`NewEnumerator0`
                                                      (switch `int` _options_index_7
                                                        (:`0`
                                                          (bind (_state_8 _options_index_8) (`self.adddialogue` "Laz" "I am going to act like you didn't say that. Any idea where Andras could even be located?" (`|MakeArray` "Continue" :!type "Text")))
                                                          (switch `/Game/ryan_stuff/Ryan_DialogueStuff/Enum_Dialoguestate` _state_8
                                                            (:`NewEnumerator0`
                                                              (switch `int` _options_index_8
                                                                (:`0`
                                                                  (bind (_state_9 _options_index_9) (`self.adddialogue` "Stevens" "A decaying lab about 15 miles west of here. Plenty of dead humans and Ashen around the area for him to reanimate, and way to much lightning coming from the roof for it to not be the location. " (`|MakeArray` "handle things" :!type "Text")))
                                                                  (switch `/Game/ryan_stuff/Ryan_DialogueStuff/Enum_Dialoguestate` _state_9
                                                                    (:`NewEnumerator0`
                                                                      (switch `int` _options_index_9
                                                                        (:`0`
                                                                          (bind (_state_10 _options_index_10) (`self.adddialogue` "Laz" "Alright, I'll handle things over there with him. Hopefully this is the last time I have to deal with him. " (`|MakeArray` "Continue" :!type "Text")))
                                                                          (switch `/Game/ryan_stuff/Ryan_DialogueStuff/Enum_Dialoguestate` _state_10
                                                                            (:`NewEnumerator0`
                                                                              (switch `int` _options_index_10
                                                                                (:`0`
                                                                                  (bind (_state_11 _options_index_11) (`self.adddialogue` "Stevens" "We'll try to handle ourselves without the protecter here. As long as you stop him Lazarus we should be okay here if thats what is slowing you down. " (`|MakeArray` "Alright" :!type "Text")))
                                                                                  (switch `/Game/ryan_stuff/Ryan_DialogueStuff/Enum_Dialoguestate` _state_11
                                                                                    (:`NewEnumerator0`
                                                                                      (switch `int` _options_index_11
                                                                                        (:`0`
                                                                                          (bind (_state_12 _options_index_12) (`self.adddialogue` "Laz" "Alrighty then, I'm holding you to that Stevens, you all better be here when I come back. " (`|MakeArray` "Continue" :!type "Text")))
                                                                                          (switch `/Game/ryan_stuff/Ryan_DialogueStuff/Enum_Dialoguestate` _state_12
                                                                                            (:`NewEnumerator0`
                                                                                              (switch `int` _options_index_12
                                                                                                (:`0`
                                                                                                  (bind (_state_13 _options_index_13) (`self.adddialogue` "Stevens" "We will be. Oh and one more thing before you go. Heavy is the crown of the one who bears more pain than he should." (`|MakeArray` "close" :!type "Text")))
                                                                                                  (switch `/Game/ryan_stuff/Ryan_DialogueStuff/Enum_Dialoguestate` _state_13
                                                                                                    (:`NewEnumerator0`
                                                                                                      (switch `int` _options_index_13
                                                                                                        (:`0`
                                                                                                          (`self.closeconversation`))))))))))))))))))))))))))))))))))))))))))))))))))))))